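; BP_Item is an item Blueprint that highlights itself and shows a text label while the player character is nearby.
; On BeginPlay it creates a UI_ItemText widget, fills it with its focus text, assigns it to the Widget component and hides it.
; Sphere overlaps with player 0's character toggle both the widget's visibility and the static mesh's Custom Depth rendering, presumably feeding an outline material.
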(event `self.ReceiveBeginPlay`
  (bind _returnvalue (`|CreateWidget` "/Game/Resouce/OutLineMaterial/UI_ItemText.UI_ItemText_C"))
  (bind _output_get (set `self.FocusTextWidget` _returnvalue))
  (`WidgetComponent.SetWidget` (`self.Widget`) _output_get)
  (`/Game/Resouce/OutLineMaterial/UI_ItemText.SetItemText` _output_get (`self.Focus Text_0`))
  (`SceneComponent.SetVisibility` (`self.Widget`) false false))

(event `self.Sphere.OnComponentBeginOverlap`
  (params (OverlappedComponent :type "PrimitiveComponent Object Reference") (OtherActor :type "Actor Object Reference") (OtherComp :type "PrimitiveComponent Object Reference") (OtherBodyIndex :type Integer) (bFromSweep :type Boolean) (SweepResult :type "HitResult Structure (by ref)"))
  (if (== OtherActor (`GameplayStatics.GetPlayerCharacter` 0))
    (`SceneComponent.SetVisibility` (`self.Widget`) true false)
    (`PrimitiveComponent.SetRenderCustomDepth` (`self.StaticMesh`) true)))

(event `self.Sphere.OnComponentEndOverlap`
  (params (OverlappedComponent :type "PrimitiveComponent Object Reference") (OtherActor :type "Actor Object Reference") (OtherComp :type "PrimitiveComponent Object Reference") (OtherBodyIndex :type Integer))
  (if (== OtherActor (`GameplayStatics.GetPlayerCharacter` 0))
    (`SceneComponent.SetVisibility` (`self.Widget`) false false)
    (`PrimitiveComponent.SetRenderCustomDepth` (`self.StaticMesh`) false)))

(fn `UserConstructionScript`)