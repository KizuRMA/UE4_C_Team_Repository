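; Camera manager Blueprint that rotates through an array of 2D scene capture actors so they take turns being active.
; BeginPlay deactivates the capture component on each entry in Cameras while keeping the one at index Num active.
; Every Tick deactivates the current capture, advances Num with wraparound and activates the next, a round-robin that spreads capture work across frames.
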(event `self.ReceiveBeginPlay`
  (bind _cameras (`self.cameras`))
  (for (_array_element _array_index) _cameras
    (`ActorComponent.SetActive` (`SceneCapture2D.CaptureComponent2D` _array_element) false false)
    (`ActorComponent.SetActive` (`SceneCapture2D.CaptureComponent2D` (`|GetArrayItem` _cameras (`self.num`))) true false)))

(event `self.ReceiveTick`
  (params (DeltaSeconds :type "Float (single-precision)"))
  (`ActorComponent.SetActive` (`SceneCapture2D.CaptureComponent2D` (`|GetArrayItem` (`self.cameras`) (`self.num`))) false false)
  (`/Engine/EditorBlueprintResources/StandardMacros.IncrementInt` (`self.num`)
    (:`  `
      (if (<= (`KismetArrayLibrary.Array_Length` (`self.cameras`)) (`self.num`))
        (set `self.num` 0))
      (`ActorComponent.SetActive` (`SceneCapture2D.CaptureComponent2D` (`|GetArrayItem` (`self.cameras`) (`self.num`))) true false))))

(fn `UserConstructionScript`)