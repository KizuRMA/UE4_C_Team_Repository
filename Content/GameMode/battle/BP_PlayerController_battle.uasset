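; Player controller for the battle game mode that creates and updates the battle HUD.
; On BeginPlay it creates WBP_UI_battle, adds it to the viewport and fills in the score from BP_PlayerState_battle.
; The score text is refreshed every Tick, while a separate DamageEventUI event pushes the player state's HP into the HP bar.
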(event `self.ReceiveBeginPlay`
  (`self.CreateWidgetOnClient`)
  (`self.UpdateUIOnClient`))

(event `self.ReceiveTick`
  (params (DeltaSeconds :type "Float (single-precision)"))
  (`self.UpdateUIOnClient`))

(event `CreateWidgetOnClient`
  (bind _returnvalue (`|CreateWidget` "/Game/GameMode/battle/WBP_UI_battle.WBP_UI_battle_C" self))
  (bind _output_get (set `self.UI` _returnvalue))
  (`UserWidget.AddToViewport` _output_get 0))

(event `UpdateUIOnClient`
  ;[1 1 1] スコア表示
  (bind _asbp_player_state_battle (cast `/Game/GameMode/battle/BP_PlayerState_battle` (`self.PlayerState`)))
  (`TextBlock.SetText` (`/Game/GameMode/battle/WBP_UI_battle.score` (`self.UI`)) (`KismetTextLibrary.Conv_IntToText` (`/Game/GameMode/battle/BP_PlayerState_battle.NowScore` _asbp_player_state_battle) false true 3)))

(event `DamageEventUI`
  ;[1 1 1] 体力表示
  (bind _asbp_player_state_battle (cast `/Game/GameMode/battle/BP_PlayerState_battle` (`self.PlayerState`)))
  (`/Game/Scene/UI/WBP_HPBar.UpdateProgress` (`/Game/GameMode/battle/WBP_UI_battle.WBP_HPBar` (`self.UI`)) (`KismetMathLibrary.Conv_IntToDouble` (`/Game/GameMode/battle/BP_PlayerState_battle.HP` _asbp_player_state_battle))))

(fn `UserConstructionScript`)