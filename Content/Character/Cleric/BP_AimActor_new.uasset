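; Aim marker actor for the Cleric that follows the owner camera's view and records a location for creating magic.
; On BeginPlay and every Tick, it line-traces along the camera forward and moves itself to the result.
; A hit places it on the impact point, oriented to the surface normal, and sets the magic location there.
; A miss leaves it at the ray end, while a downward trace seeks ground for the magic location.
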(event `self.ReceiveBeginPlay`
  (`self.Camera Look Trace`)
  (`self.K2_SetActorTransform` (`KismetMathLibrary.MakeTransform` (`self.Aim Actor Location`) (`SceneComponent.K2_GetComponentRotation` (`self.Owner Camera`)) (2.0 2.0 2.0))))

(event `self.ReceiveTick`
  (params (DeltaSeconds :type "Float (single-precision)"))
  (`self.Camera Look Trace`)
  (`self.K2_SetActorTransform` (`KismetMathLibrary.MakeTransform` (`self.Aim Actor Location`) (`self.Aim Rotator`) (2.0 2.0 2.0))))

(fn `Camera Look Trace`
  (locals (`Ray Distance` :type "Float (double-precision)" :default 1500.0) (`Ray End Location` :type "Vector Structure") (`test vector` :type "Vector Structure" :default (-1.0 0.0 0.0)) (`test 2 vector` :type "Vector Structure" :default (0.0 1.0 0.0)))
  (bind _ray_end_location (`local.Ray End Location`))
  (bind _owner_camera (`self.Owner Camera`))
  (bind _returnvalue (`SceneComponent.K2_GetComponentLocation` _owner_camera))
  (bind _returnvalue_2 (+ _returnvalue (* (`KismetMathLibrary.GetForwardVector` (`SceneComponent.K2_GetComponentRotation` _owner_camera)) (`local.Ray Distance`))))
  ;[1 1 1] カメラが向いてる方向にレイ判定
  (set `local.Ray End Location` _returnvalue_2)
  (bind (_outhit _returnvalue_3) (`KismetSystemLibrary.LineTraceSingle` :`Start` _returnvalue :`End` _returnvalue_2 :`TraceChannel` "TraceTypeQuery1" :`DrawDebugType` "ForOneFrame"))
  (if _returnvalue_3
    (bind (_bblockinghit _binitialoverlap _time _distance _location _impactpoint _normal) (`GameplayStatics.BreakHitResult` _outhit))
    ;[1 1 1] カメラの注視点にオブジェクトがあるとき
    (bind _output_get (set `self.Aim Actor Location` _location))
    (set `self.Create Magic Location` _output_get)
    (set `self.Aim Rotator` (`KismetMathLibrary.MakeRotFromXZ` _normal (`SceneComponent.GetUpVector` (`self.DefaultSceneRoot`))))
    (return)
    (else
      ;[1 1 1] 下に向かってレイ判定
      ;;[1 1 1] 下に向かってレイ判定
      (set `self.Aim Actor Location` _ray_end_location)
      (bind (_outhit_2 _returnvalue_4) (`KismetSystemLibrary.LineTraceSingle` :`Start` _ray_end_location :`End` (+ _ray_end_location (`KismetMathLibrary.MakeVector` 0.0 0.0 (* -1 (`local.Ray Distance`)))) :`TraceChannel` "TraceTypeQuery1" :`DrawDebugType` "ForOneFrame"))
      (if _returnvalue_4
        (set `self.Create Magic Location` (`.Location` (`GameplayStatics.BreakHitResult` _outhit_2)))
        (set `self.Aim Rotator` (`SceneComponent.K2_GetComponentRotation` (`self.Owner Camera`)))
        (return)))))

(fn `UserConstructionScript`)