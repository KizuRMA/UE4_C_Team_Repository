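; BP_EnemyMapArrow is an actor that, by its name, serves as a map arrow marking the direction of an enemy from player 0.
; Each tick it moves itself far out along the player-to-enemy line by scaling the unnormalized offset by a large constant.
; It destroys itself when the enemy reference becomes invalid or the horizontal distance to the player drops below a threshold.
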(event `self.ReceiveTick`
  (params (DeltaSeconds :type "Float (single-precision)"))
  (bind _returnvalue (`self.K2_GetActorLocation` (`GameplayStatics.GetPlayerCharacter` 0)))
  (bind _returnvalue_2 (- (`self.K2_GetActorLocation` (`self.Enemy`)) _returnvalue))
  (`/Engine/EditorBlueprintResources/StandardMacros.IsValid` (`self.Enemy`)
    (:`Is Valid`
      (`self.K2_SetActorLocation` (+ (* _returnvalue_2 5000.0) _returnvalue))
      (if (< (`KismetMathLibrary.VSizeXY` _returnvalue_2) 2000.0)
        (`self.K2_DestroyActor`)))
    (:`Is Not Valid`
      (`self.K2_DestroyActor`))))

(fn `UserConstructionScript`)