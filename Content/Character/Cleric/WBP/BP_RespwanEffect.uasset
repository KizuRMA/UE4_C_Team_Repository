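; BP_RespwanEffect is a respawn effect actor under the Cleric character that destroys itself when its P_ProjCore particle system finishes.
; That finish event is the only active logic, as BeginPlay and the construction script are empty.
; An unconnected timeline chain would color the core and trail, spiral them around a rotating pivot while driving alpha, then destroy the actor after a short delay.
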(event `self.ReceiveBeginPlay`)

(event `self.P_ProjCore.OnSystemFinished`
  (params (PSystem :type "ParticleSystemComponent Object Reference"))
  (`self.K2_DestroyActor`))

(fn `UserConstructionScript`)