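; GM_Player is a game mode that overrides ChoosePlayerStart to pick a spawn point based on a room member ID.
; It takes the ID from GetCurrentRoomMember and converts it through Game_Instance_Main's IDtoRoomIDConvert, printing the result.
; The converted ID serves as the tag to find a matching PlayerStart, with any PlayerStart as fallback.
; The Player argument is unused, and BeginPlay, Tick and the construction script are empty.
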(fn `ChoosePlayerStart`
  (params (Player :type "Controller Object Reference"))
  (returns (ReturnValue :type "Actor Object Reference"))
  (bind _asgame_instance_main (cast `/Game/Scene/Game_Instance_Main` (`GameplayStatics.GetGameInstance`)))
  (bind _returnvalue (`StrixBlueprintFunctionLibrary.GetCurrentRoomMember` 0))
  (bind _roomid (`/Game/Scene/Game_Instance_Main.IDtoRoomIDConvert` _asgame_instance_main (break `StrixRoomMember` _returnvalue)))
  (bind _returnvalue_2 (`KismetStringLibrary.Conv_IntToString` _roomid))
  (`KismetSystemLibrary.PrintString` _returnvalue_2)
  (bind _outactors (`GameplayStatics.GetAllActorsOfClassWithTag` "/Script/Engine.PlayerStart" (`KismetStringLibrary.Conv_StringToName` _returnvalue_2)))
  (bind _output (`|GetArrayItem` _outactors))
  (`/Engine/EditorBlueprintResources/StandardMacros.IsValid` _output
    (:`Is Valid`
      (return _output))
    (:`Is Not Valid`
      (bind _returnvalue_3 (`GameplayStatics.GetActorOfClass` "/Script/Engine.PlayerStart"))
      (return _returnvalue_3))))

(fn `UserConstructionScript`)