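; BP_EnemySpawnPoint is a spawn point that creates random enemies while players are nearby.
; Its Sphere tracks overlapping actors, toggles the near-player flag and billboard sprite, and sets the spawn radius.
; Each Tick, if Strix is offline or this client is room owner and replicator owner, it checks EnemyCheckSphere's overlap count.
; Below PopLimit, it spawns a PopEnemyList class at a random reachable point.
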(event `self.ReceiveTick`
  (params (DeltaSeconds :type "Float (single-precision)"))
  (bind _returnvalue (`StrixBlueprintFunctionLibrary.IsRoomServerConnected` 0))
  (if _returnvalue
    (bind _returnvalue_2 (`StrixBlueprintFunctionLibrary.IsRoomOwner` 0))
    (if (and _returnvalue_2 (`StrixReplicatorComponent.GetIsOwner` (`self.StrixReplicator`)))
      (if (`self.IsNearPlayer`) :!label _label
        (bind _poppossible (`self.EnemyCheck`)
          (:`NewParam2`
            (if _poppossible
              (`self.PopEnemy`)
              (`KismetSystemLibrary.PrintString` "Spawn"))))))
    (else
      (goto _label))))

(event `self.Sphere.OnComponentBeginOverlap`
  (params (OverlappedComponent :type "PrimitiveComponent Object Reference") (OtherActor :type "Actor Object Reference") (OtherComp :type "PrimitiveComponent Object Reference") (OtherBodyIndex :type Integer) (bFromSweep :type Boolean) (SweepResult :type "HitResult Structure (by ref)"))
  (if (not (`BlueprintSetLibrary.Set_Contains` (`self.NearPlayer`) OtherActor))
    (`BlueprintSetLibrary.Set_Add` (`self.NearPlayer`) OtherActor)
    (set `self.IsNearPlayer` true)
    (`BillboardComponent.SetSprite` (`self.Billboard`) "/Game/Animetion/AnimStarterPack/UE4_Mannequin/Textures/UE4_LOGO_CARD.UE4_LOGO_CARD")))

(event `self.Sphere.OnComponentEndOverlap`
  (params (OverlappedComponent :type "PrimitiveComponent Object Reference") (OtherActor :type "Actor Object Reference") (OtherComp :type "PrimitiveComponent Object Reference") (OtherBodyIndex :type Integer))
  (bind _nearplayer (`self.NearPlayer`))
  (if (`BlueprintSetLibrary.Set_Contains` (`self.NearPlayer`) OtherActor)
    (`BlueprintSetLibrary.Set_Remove` _nearplayer OtherActor)
    (if (== (`BlueprintSetLibrary.Set_Length` _nearplayer) 0)
      (set `self.IsNearPlayer` false)
      (`BillboardComponent.SetSprite` (`self.Billboard`) null))))

(fn `PopEnemy`
  (`|SpawnActorFromClass` (`KismetArrayLibrary.Array_Random` (`self.PopEnemyList`)) (`KismetMathLibrary.MakeTransform` (`NavigationSystemV1.K2_GetRandomReachablePointInRadius` (`self.K2_GetActorLocation`) (`SphereComponent.SphereRadius` (`self.Sphere`)) null null)) "Undefined" "OverrideRootScale" null null))

(fn `UserConstructionScript`)