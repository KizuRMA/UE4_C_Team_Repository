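; Slime enemy character that plays a near-attack montage and damages a BP_Cleric_new player on hit, with parallel Local and Strix network-owner overrides.
; Animation functions toggle the attack window and Flying/Walking for jumps; a hit closes the window.
; Only the local hit uses DamageNear and ends the jump; the Strix hit hardcodes damage.
; Timelines fade opacity on spawn and death, and the HP widget attaches to a mesh socket.
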(event `self.ReceiveBeginPlay`
  (`parent.ReceiveBeginPlay`)
  (bind (_direction _opacity) (`Timeline|タイムライン_0`)
    (:`Update`
      (`MeshComponent.SetScalarParameterValueOnMaterials` (`self.Mesh`) "Opacity" _opacity))))

(event `Animetion_Down`
  (bind _mesh (`self.Mesh`))
  (`PrimitiveComponent.SetCastShadow` _mesh false)
  (`PrimitiveComponent.SetCollisionEnabled` _mesh "NoCollision")
  (bind (_direction _opacity) (`Timeline|DownTimeLine`)
    (:`Update`
      (`MeshComponent.SetScalarParameterValueOnMaterials` (`self.Mesh`) "Opacity" _opacity))
    (:`Finished`
      (bind _networktype (`self.Select`))
      (switch `/Game/Character/NetworkType` _networktype
        (:`NewEnumerator0`
          _)
        (:`NewEnumerator2`
          _))
      (`self.K2_DestroyActor`))))

(fn `Animetion_Attack_End`
  (set `self.IsAttacking` false))

(fn `Animetion_Attack_Start`
  (set `self.IsAttacking` true))

(fn `Animetion_Jump_End`
  (`CharacterMovementComponent.SetMovementMode` (`self.CharacterMovement`) "MOVE_Walking" 0))

(fn `Animetion_Jump_Start`
  (`CharacterMovementComponent.SetMovementMode` (`self.CharacterMovement`) "MOVE_Flying" 0))

(fn `AttackFunction_Local`
  (params (playerControllerID :type Integer) (DamagePoint :type Integer))
  (`self.PlayAnimMontage` (`self.AttackMontage_near`)))

(fn `AttackFunction_Owner_Strix`
  (params (playerControllerID :type Integer) (DamagePoint :type Integer) (IsRoomOwner :type Boolean))
  (`self.PlayAnimMontage` (`self.AttackMontage_near`)))

(fn `BeginFunction_Local`
  (`parent.BeginFunction_Local`)
  (`SceneComponent.K2_AttachToComponent` (`self.HPWidget`) (`self.Mesh`) "TargetHp" "KeepWorld" "SnapToTarget" "SnapToTarget" true))

(fn `BeginFunction_Owner_Strix`
  (params (IsRoomOwner :type Boolean))
  (`parent.BeginFunction_Owner_Strix` false)
  (`SceneComponent.K2_AttachToComponent` (`self.HPWidget`) (`self.Mesh`) "TargetHp" "KeepWorld" "SnapToTarget" "SnapToTarget" true))

(fn `HitFunction_Local`
  (params (HitActor :type "Actor Object Reference") (HitLocation :type "Vector Structure"))
  (if (`self.ActorHasTag` HitActor "Player")
    (if (`self.IsAttacking`)
      (bind _asbp_cleric_new (cast `/Game/Character/Cleric/BP_Cleric_new` HitActor))
      (`self.Damaged` _asbp_cleric_new (`self.Damage_near`) 0 0 (`self.K2_GetActorLocation`) "NewEnumerator0")
      (set `self.IsAttacking` false)
      (`self.Animetion_Jump_End`))))

(fn `HitFunction_Owner_Strix`
  (params (HitActor :type "Actor Object Reference") (HitLocation :type "Vector Structure") (IsRoomOwner :type Boolean))
  (if (`self.ActorHasTag` HitActor "Player")
    (if (`self.IsAttacking`)
      (bind _asbp_cleric_new (cast `/Game/Character/Cleric/BP_Cleric_new` HitActor))
      (`self.Damaged` _asbp_cleric_new 3 0 0 (`self.K2_GetActorLocation`) "NewEnumerator0")
      (set `self.IsAttacking` false))))

(fn `UserConstructionScript`
  (`parent.UserConstructionScript`))