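; Base enemy Blueprint with elemental damage, HP bar, lock-on marker and distance-based despawn, for local or Strix network play.
; Local, Owner and Client functions set up widgets and apply damage, updating the bar and spawning damage numbers.
; At zero HP, DeathFunction awards score, randomly drops a magic stone, notifies the AI and plays the death montage, via RPC for Owner.
; Tick billboards the HP bar and distance-culls it once damaged.
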(event `SetElementIcon`
  (params (type :type Byte))
  (bind _aswbp_hpbar_enemy (cast `/Game/Character/Enemy/WBP_HPBar_enemy` (`WidgetComponent.GetWidget` (`self.HPWidget`))))
  (`/Game/Character/Enemy/WBP_HPBar_enemy.setElementIcon` _aswbp_hpbar_enemy type))

(event `/Game/Cleric/Blueprints/Interfarce/BP_CharacterIntarface.SetLockOnState`
  (params (Enable :type Boolean))
  (bind _mesh (`self.Mesh`))
  (`SceneComponent.SetVisibility` (`self.RockOnMarker`) Enable false)
  (`PrimitiveComponent.SetRenderCustomDepth` (`self.Mesh`) Enable)
  (if Enable
    (`PrimitiveComponent.SetCustomDepthStencilValue` _mesh 1)
    (`PrimitiveComponent.SetCustomDepthStencilValue` (`self.Mesh`) 1)
    (else
      (`PrimitiveComponent.SetCustomDepthStencilValue` _mesh 0))))

(event `Despawn`
  ;[1 1 1] デスポーン処理（GetAllActorを使っているためinitで呼び出す）
  (`self.Select_Macro` :!label _label
    (:`Local`
      _)
    (:`Owner`
      _))
  (bind _newparam (`self.Despawn Check`))
  (if _newparam
    (`self.K2_DestroyActor`)
    (else
      (`KismetSystemLibrary.Delay` 3.0)
      (goto _label))))

(event `DeathFunction`
  (`KismetSystemLibrary.Delay` 0.2)
  (`|ExecutionSequence`
    (:`then_0`
      ;[1 1 1] スコア加算処理
      (if (not (`self.IsDeath`))
        (set `self.IsDeath` true)
        (bind _actor (`self.Actor`)
          (:`then`
            (message `/Game/Cleric/Blueprints/Interfarce/BP_CharacterIntarface.AddScore_i` _actor (`self.SCORE`))
            ;[1 1 1] 戦闘
            (bind _asbp_cleric_new (cast `/Game/Character/Cleric/BP_Cleric_new` _actor))
            (`/Game/Character/Cleric/BP_Cleric_new.RemoveFinder` _asbp_cleric_new self))
          (:`else`))))
    (:`then_1`
      ;[1 1 1] 魔石ドロップ
      (if (> (`self.DropProbability`) (`KismetMathLibrary.RandomInteger` 100))
        (bind _returnvalue (`|GetDataTableRow` "/Game/DataTable/DT_MagicDefineTable.DT_MagicDefineTable" (`KismetArrayLibrary.Array_Random` (`self.DropMagicStoneType`)))
          (:`then`
            (`|SpawnActorFromClass` "/Game/Magic/MagicStone/Blueprint/BP_MagicStoneBase.BP_MagicStoneBase_C" (`KismetMathLibrary.MakeTransform` (`self.K2_GetActorLocation`)) "Undefined" "OverrideRootScale" null (`.MagicInfoDifine_36_69F1A7CE4DA11F35F152749B8340C8A0` (break `/Game/DataTable/Struct/S_MagicDifine` _returnvalue)) null)))))
    (:`then_2`
      (bind _asaic_enemy_base (cast `/Game/Character/Enemy/Base/AIC_EnemyBase` (`AIBlueprintHelperLibrary.GetAIController` self)))
      (`/Game/Character/Enemy/Base/AIC_EnemyBase.Set Alive Flg` _asaic_enemy_base false)
      (`self.Select_Macro`
        (:`Local`
          (`self.DethAnimetionStart`))
        (:`Owner`
          (`StrixBlueprintFunctionLibrary.SendRpcToAll` null "DethAnimetionStart"))))
    (:`then_3`
      (bind _asaic_enemy_base_2 (cast `/Game/Character/Enemy/Base/AIC_EnemyBase` (`AIBlueprintHelperLibrary.GetAIController` self)))
      (`/Game/Character/Enemy/Base/AIC_EnemyBase.Sound Destory` _asaic_enemy_base_2))))

(event `self.ReceiveTick`
  (params (DeltaSeconds :type "Float (single-precision)"))
  (`|ExecutionSequence`
    (:`then_0`
      (if (!= (`self.HP`) (`self.MAXHP`))
        (`SceneComponent.SetVisibility` (`self.HPWidget`) (< (`KismetMathLibrary.VSize` (- (`self.K2_GetActorLocation` (`GameplayStatics.GetPlayerCharacter` 0)) (`self.K2_GetActorLocation`))) 3000.0) false)))
    (:`then_1`
      (`self.Set BIll`))))

(event `Set BIll`
  (bind _hpwidget (`self.HPWidget`))
  (`SceneComponent.K2_SetWorldRotation` _hpwidget (`KismetMathLibrary.FindLookAtRotation` (`SceneComponent.K2_GetComponentLocation` _hpwidget) (`PlayerCameraManager.GetCameraLocation` (`GameplayStatics.GetPlayerCameraManager` 0))) false false))

(fn `Add Magic ID`
  (params (ID :type Integer))
  (bind _asgame_instance_main (cast `/Game/Scene/Game_Instance_Main` (`GameplayStatics.GetGameInstance`)))
  (bind _now_time (`/Game/Scene/Game_Instance_Main.Get Progress Time` _asgame_instance_main))
  (for _array_element (`self.MagicID`)
    (bind _magicid (break `/Game/Character/Enemy/S_EnemyDamaged` _array_element))
    (if (== _magicid ID)
      (setmembers `/Game/Character/Enemy/S_EnemyDamaged` :`StructRef` _array_element :`MagicID` _magicid :`Previous Damage Time` _now_time)
      (return)))
  (`KismetArrayLibrary.Array_Add` (`self.MagicID`) (make `/Game/Character/Enemy/S_EnemyDamaged` ID _now_time))
  (`KismetSystemLibrary.PrintString` "追加しました" true true (struct :`R` 1.0 :`B` 0.090672 :`A` 1.0))
  (return))

(fn `BeginFunction_Client_Strix`
  (params (IsRoomOwner :type Boolean))
  (`SceneComponent.K2_AttachToComponent` (`self.RockOnMarker`) (`self.Mesh`) "TargetSocket" "SnapToTarget" "SnapToTarget" "SnapToTarget" true)
  (bind _aswbp_hpbar_enemy (cast `/Game/Character/Enemy/WBP_HPBar_enemy` (`WidgetComponent.GetWidget` (`self.HPWidget`))))
  (`/Game/Character/Enemy/WBP_HPBar_enemy.Init` _aswbp_hpbar_enemy (`self.HP`)))

(fn `BeginFunction_Local`
  (bind _rockonmarker (`self.RockOnMarker`))
  (bind (_returnvalue_x _returnvalue_y) (`KismetMathLibrary.BreakVector2D` (`WidgetComponent.GetDrawSize` _rockonmarker)))
  (`SceneComponent.K2_AttachToComponent` (`self.RockOnMarker`) (`self.Mesh`) "TargetSocket" "SnapToTarget" "SnapToTarget" "SnapToTarget" true)
  (bind _aswbp_hpbar_enemy (cast `/Game/Character/Enemy/WBP_HPBar_enemy` (`WidgetComponent.GetWidget` (`self.HPWidget`))))
  (`/Game/Character/Enemy/WBP_HPBar_enemy.Init` _aswbp_hpbar_enemy (`self.HP`))
  (`self.SetElementIcon` (`self.MyElementType`))
  (`self.Despawn`)
  (bind _asw_target_mark (cast `/Game/UI/Cleric_UI/W_TargetMark` (`WidgetComponent.GetWidget` _rockonmarker)))
  (`/Game/UI/Cleric_UI/W_TargetMark.SetScale` _asw_target_mark _returnvalue_x _returnvalue_y)
  (bind _aswbp_hpbar_enemy_2 (cast `/Game/Character/Enemy/WBP_HPBar_enemy` (`WidgetComponent.GetWidget` (`self.HPWidget`))))
  (set `/Game/Character/Enemy/WBP_HPBar_enemy.Enemy` self _aswbp_hpbar_enemy_2))

(fn `BeginFunction_Owner_Strix`
  (params (IsRoomOwner :type Boolean))
  (`|ExecutionSequence`
    (:`then_0`
      (bind _hpwidget (`self.HPWidget`)
        (:`then`
          (bind _aswbp_hpbar_enemy (cast `/Game/Character/Enemy/WBP_HPBar_enemy` (`WidgetComponent.GetWidget` _hpwidget)))
          (`/Game/Character/Enemy/WBP_HPBar_enemy.Init` _aswbp_hpbar_enemy (`self.HP`))
          (`StrixBlueprintFunctionLibrary.SendRpcToAll` null "SetElementIcon" (`|MakeArray` (`StrixBlueprintFunctionLibrary.Conv_ByteToStrixRelayArg` (`self.MyElementType`))))
          (bind _aswbp_hpbar_enemy_2 (cast `/Game/Character/Enemy/WBP_HPBar_enemy` (`WidgetComponent.GetWidget` (`self.HPWidget`))))
          (set `/Game/Character/Enemy/WBP_HPBar_enemy.Enemy` self _aswbp_hpbar_enemy_2))
        (:`else`)))
    (:`then_1`
      (bind _rockonmarker (`self.RockOnMarker`)
        (:`then`
          (`self.Despawn`)
          (bind _asw_target_mark (cast `/Game/UI/Cleric_UI/W_TargetMark` (`WidgetComponent.GetWidget` _rockonmarker)))
          (bind (_returnvalue_x _returnvalue_y) (`KismetMathLibrary.BreakVector2D` (`WidgetComponent.GetDrawSize` _rockonmarker)))
          (`/Game/UI/Cleric_UI/W_TargetMark.SetScale` _asw_target_mark _returnvalue_x _returnvalue_y)
          (`SceneComponent.K2_AttachToComponent` (`self.RockOnMarker`) (`self.Mesh`) "TargetSocket" "SnapToTarget" "SnapToTarget" "SnapToTarget" true))
        (:`else`)))))

(fn `DamageFunction_Local`
  (params (DamagePoint :type Integer) (playerControllerID :type Integer) (TargetActorLocation :type "Vector Structure") (ElementNumber :type Byte) (Critical :type Boolean))
  (bind _returnvalue (cast `/Game/Character/Magic/Data/ElementType` ElementNumber))
  (if (not (`self.IsDeath`))
    (bind (_hp _calcdamage _compatibility) (`self.DamageCalc` DamagePoint _returnvalue))
    (bind _aswbp_hpbar_enemy (cast `/Game/Character/Enemy/WBP_HPBar_enemy` (`WidgetComponent.GetWidget` (`self.HPWidget`))))
    (`/Game/Character/Enemy/WBP_HPBar_enemy.HPUpdate` _aswbp_hpbar_enemy _hp)
    (`self.damageView` _calcdamage _returnvalue _compatibility Critical)))

(fn `DamageFunction_Owner_Strix`
  (params (DamagePoint :type Integer) (RoomMenberID :type Integer) (IsRoomOwner :type Boolean) (TargetActorLocation :type "Vector Structure") (ElementType :type Byte) (Critical :type Boolean))
  (bind _returnvalue (cast `/Game/Character/Magic/Data/ElementType` ElementType))
  (if (not (`self.IsDeath`))
    (bind (_hp _calcdamage _compatibility) (`self.DamageCalc` DamagePoint _returnvalue))
    (bind _aswbp_hpbar_enemy (cast `/Game/Character/Enemy/WBP_HPBar_enemy` (`WidgetComponent.GetWidget` (`self.HPWidget`))))
    (`/Game/Character/Enemy/WBP_HPBar_enemy.HPUpdate` _aswbp_hpbar_enemy _hp)
    (`self.damageView` _calcdamage _returnvalue _compatibility Critical)))

(fn `damageView`
  (params (damage :type Integer) (Selection :type "/Game/Character/Magic/Data/ElementType Enum" :default "NewEnumerator0") (ElementIndex :type "/Game/Character/Magic/Data/ElementIndex Enum" :default "NewEnumerator0") (Critical :type Boolean))
  (locals (color :type "SlateColor Structure") (size :type Integer))
  (bind _returnvalue (`|SpawnActorFromClass` "/Enemy/Enemy/BP/BP_damageView.BP_damageView_C" (`KismetMathLibrary.MakeTransform` (`SceneComponent.GetSocketLocation` (`self.Mesh`) "TargetSocket")) "Undefined" "OverrideRootScale" null null))
  (`/Enemy/Enemy/BP/BP_damageView.setText` _returnvalue damage Selection ElementIndex Critical))

(fn `DeathFunction_Local`
  (params (playerControllerID :type Integer)))

(fn `DeathFunction_Owner_Strix`
  (params (RoomMenberID :type Integer)))

(fn `Despawn Check`
  (returns (NewParam :type Boolean))
  (locals (nearDis :type "Float (double-precision)" :default 1.0000000200408773e+20))
  (`|ExecutionSequence`
    (:`then_0`
      (`/Engine/EditorBlueprintResources/StandardMacros.DoOnce` false
        (:`Completed`
          (bind _outactors (`GameplayStatics.GetAllActorsOfClass` "/Game/Character/Cleric/BP_Cleric_new.BP_Cleric_new_C"))
          (set `self.player` _outactors))))
    (:`then_1`
      (for _array_element (`self.player`)
        (bind _returnvalue (`KismetMathLibrary.VSize` (- (`self.K2_GetActorLocation` _array_element) (`self.K2_GetActorLocation`))))
        (if (< _returnvalue (`local.nearDis`))
          (set `local.nearDis` _returnvalue)))
      (return (>= (`local.nearDis`) (`self.DespawnDistance`))))))

(fn `DethAnimetionStart`
  (`self.PlayAnimMontage` (`self.DeathMontage`))
  (`PrimitiveComponent.SetCollisionEnabled` (`self.CapsuleComponent`) "NoCollision")
  (`PrimitiveComponent.SetCollisionEnabled` (`self.Mesh`) "NoCollision"))

(fn `Find Magic Hit TIme`
  (params (ID :type Integer))
  (returns (TIme :type "Float (double-precision)") (Hit :type Boolean))
  (for _array_element (`self.MagicID`)
    (bind (_magicid _previousdamagetime) (break `/Game/Character/Enemy/S_EnemyDamaged` _array_element))
    (if (== _magicid ID)
      (return _previousdamagetime true)))
  (return 0.0 false))

(fn `HP_Update_Timing`
  (params (hp :type Integer))
  (if (<= hp 0)
    (`self.DeathFunction`)
    (else
      (set `self.Actor` null))))

(fn `OnRep_actor`)

(fn `SetStrixFunction`
  (`parent.SetStrixFunction`)
  (`StrixBlueprintFunctionLibrary.RegisterStrixRpc` null "DethAnimetionStart")
  (`StrixBlueprintFunctionLibrary.RegisterStrixRpc` null "SetElementIcon"))

(fn `UserConstructionScript`
  (`parent.UserConstructionScript`))