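; Dragon enemy Blueprint with near and far attacks, supporting local and Strix-networked play.
; A flag, set by an event registered as a Strix RPC, selects the near or far montage.
; Fire spawns a breath actor between two mouth sockets, aimed at the blackboard TargetPoint, only in Local or Owner mode.
; Animation start/end functions gate single-hit damage on the Cleric player, using DamageNear locally but a hardcoded value for the Strix owner.
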(event `IsFarAttack`
  (params (`far Attack` :type Boolean))
  (set `self.IsFarAttackFlg` `far Attack`))

(event `Fire`
  (bind _mesh (`self.Mesh`))
  (bind _returnvalue (/ (+ (`SceneComponent.GetSocketLocation` _mesh "BreathPoint_upper") (`SceneComponent.GetSocketLocation` _mesh "BreathPoint_under")) 2.0))
  (bind _networktype (`self.Select`))
  (switch `/Game/Character/NetworkType` _networktype
    (:`NewEnumerator0`
      _)
    (:`NewEnumerator2`
      _))
  (bind _returnvalue_2 (`|SpawnActorFromClass` "/Game/Character/Magic/BP_Magic/BP_DragonBreath_new.BP_DragonBreath_new_C" (`KismetMathLibrary.MakeTransform` _returnvalue) "Undefined" "OverrideRootScale" self "DragonBreath" 0 self))
  (`/Game/Character/Magic/BP_Magic/BP_MagicBase_new.Init` _returnvalue_2 (`BlackboardComponent.GetValueAsVector` (`AIBlueprintHelperLibrary.GetBlackboard` null) "TargetPoint") _returnvalue))

(fn `Animetion Attack End`
  (set `self.IsAttacking` false))

(fn `Animetion_Attack_Start`
  (set `self.IsAttacking` true))

(fn `AttackFunction_Local`
  (params (playerControllerID :type Integer) (DamagePoint :type Integer))
  (if (`self.IsFarAttackFlg`)
    (`self.PlayAnimMontage` (`self.AttackMontage_far`))
    (else
      (`self.PlayAnimMontage` (`self.AttackMontage_near`)))))

(fn `AttackFunction_Owner_Strix`
  (params (playerControllerID :type Integer) (DamagePoint :type Integer) (IsRoomOwner :type Boolean))
  (if (`self.IsFarAttackFlg`)
    (`self.PlayAnimMontage` (`self.AttackMontage_far`))
    (else
      (`self.PlayAnimMontage` (`self.AttackMontage_near`)))))

(fn `HitFunction_Local`
  (params (HitActor :type "Actor Object Reference") (HitLocation :type "Vector Structure"))
  (if (`self.ActorHasTag` HitActor "Player")
    (if (`self.IsAttacking`)
      (bind _asbp_cleric_new (cast `/Game/Character/Cleric/BP_Cleric_new` HitActor))
      (`self.Damaged` _asbp_cleric_new (`self.Damage_near`) 0 0 (0.0 0.0 0.0))
      (set `self.IsAttacking` false))))

(fn `HitFunction_Owner_Strix`
  (params (HitActor :type "Actor Object Reference") (HitLocation :type "Vector Structure") (IsRoomOwner :type Boolean))
  (if (`self.ActorHasTag` HitActor "Player")
    (if (`self.IsAttacking`)
      (bind _asbp_cleric_new (cast `/Game/Character/Cleric/BP_Cleric_new` HitActor))
      (`self.Damaged` _asbp_cleric_new 6 0 0 (0.0 0.0 0.0))
      (set `self.IsAttacking` false))))

(fn `SetStrixFunction`
  (`parent.SetStrixFunction`)
  (`StrixBlueprintFunctionLibrary.RegisterStrixRpc` null "IsFarAttack"))

(fn `UserConstructionScript`
  (`parent.UserConstructionScript`))