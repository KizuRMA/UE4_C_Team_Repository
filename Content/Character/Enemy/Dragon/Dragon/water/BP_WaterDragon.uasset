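; Water dragon enemy Blueprint that handles a three-rock spread attack and the death dissolve.
; RockSkip spawns BP_DragonRock projectiles at the mesh socket and launches them in a randomized center, right and left fan, using CalcVec for the base velocity.
; Animetion_Down disables mesh shadow and collision, then a timeline drives the material Rate parameter before the actor is destroyed.
; Spawning and destruction run only for the Local or Owner network type.
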(event `RockSkip`
  (bind _returnvalue (+ (`SceneComponent.GetSocketLocation` (`self.Mesh`) "RockSkip") (0.0 0.0 -5.0)))
  (bind _networktype (`self.Select`))
  (switch `/Game/Character/NetworkType` _networktype
    (:`NewEnumerator0`
      _)
    (:`NewEnumerator2`
      _))
  (for _index (range 3)
    (bind _returnvalue_2 (`|SpawnActorFromClass` "/Game/Character/Magic/BP_Magic/BP_DragonRock.BP_DragonRock_C" (`KismetMathLibrary.MakeTransform` _returnvalue) "Undefined" "OverrideRootScale" self "DragonRock" 0 self))
    (`/Game/Character/Magic/BP_Magic/BP_MagicBase_new.Init` _returnvalue_2 (0.0 0.0 0.0) _returnvalue)
    (bind _projectilemovement (`/Game/Character/Magic/BP_Magic/BP_MagicBase_new.ProjectileMovement` _returnvalue_2)
      (:`then`
        (switch `int` _index
          (:`0`
            (set `MovementComponent.Velocity` (`KismetMathLibrary.GreaterGreater_VectorRotator` (`self.CalcVec`) (`KismetMathLibrary.MakeRotator` 0.0 0.0 (`KismetMathLibrary.RandomFloatInRange` -2.0 2.0))) _projectilemovement))
          (:`1`
            (set `MovementComponent.Velocity` (`KismetMathLibrary.GreaterGreater_VectorRotator` (`self.CalcVec`) (`KismetMathLibrary.MakeRotator` 0.0 0.0 (`KismetMathLibrary.RandomFloatInRange` 5.0 7.0))) _projectilemovement))
          (:`2`
            (set `MovementComponent.Velocity` (`KismetMathLibrary.GreaterGreater_VectorRotator` (`self.CalcVec`) (`KismetMathLibrary.MakeRotator` 0.0 0.0 (`KismetMathLibrary.RandomFloatInRange` -7.0 -5.0))) _projectilemovement))))
      (:`else`))))

(event `Animetion_Down`
  (bind _mesh (`self.Mesh`))
  (`PrimitiveComponent.SetCastShadow` _mesh false)
  (`PrimitiveComponent.SetCollisionEnabled` _mesh "NoCollision")
  (bind (_direction _rate) (`Timeline|タイムライン_0`)
    (:`Update`
      (`MeshComponent.SetScalarParameterValueOnMaterials` (`self.Mesh`) "Rate" _rate))
    (:`Finished`
      (bind _networktype (`self.Select`))
      (switch `/Game/Character/NetworkType` _networktype
        (:`NewEnumerator0`
          _)
        (:`NewEnumerator2`
          _))
      (`self.K2_DestroyActor`))))

(fn `UserConstructionScript`
  (`parent.UserConstructionScript`))