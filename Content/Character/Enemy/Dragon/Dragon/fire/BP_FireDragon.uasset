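; BP_FireDragon is the fire dragon enemy character, adding spawn fade, breath attack and death presentation to its parent.
; On BeginPlay a timeline drives material opacity, then swaps in the red material.
; Fire spawns a breath actor between two mouth sockets, aimed at the blackboard's TargetPoint, for Local or Owner network types.
; Death picks a flying or normal montage; Animetion_Down disables collision and shadows, animates a material Rate, then destroys the actor.
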(event `self.ReceiveBeginPlay`
  (`parent.ReceiveBeginPlay`)
  (bind (_direction _opacity) (`Timeline|タイムライン_1`)
    (:`Update`
      (`MeshComponent.SetScalarParameterValueOnMaterials` (`self.Mesh`) "opacity" _opacity))
    (:`Finished`
      (`PrimitiveComponent.SetMaterial` (`self.Mesh`) 0 "/Enemy/Dragon/material/RedMat_Inst.RedMat_Inst"))))

(event `Fire`
  (bind _mesh (`self.Mesh`))
  (bind _returnvalue (/ (+ (`SceneComponent.GetSocketLocation` _mesh "BreathPoint_upper") (`SceneComponent.GetSocketLocation` _mesh "BreathPoint_under")) 2.0))
  (bind _networktype (`self.Select`))
  (switch `/Game/Character/NetworkType` _networktype
    (:`NewEnumerator0`
      _)
    (:`NewEnumerator2`
      _))
  (bind _returnvalue_2 (`|SpawnActorFromClass` "/Game/Character/Magic/BP_Magic/BP_DragonBreath_new.BP_DragonBreath_new_C" (`KismetMathLibrary.MakeTransform` _returnvalue) "Undefined" "OverrideRootScale" self "DragonBreath" 0 self))
  (`/Game/Character/Magic/BP_Magic/BP_MagicBase_new.Init` _returnvalue_2 (`BlackboardComponent.GetValueAsVector` (`AIBlueprintHelperLibrary.GetBlackboard` null) "TargetPoint") _returnvalue))

(event `Animetion_Down`
  (bind _mesh (`self.Mesh`))
  (`PrimitiveComponent.SetCastShadow` _mesh false)
  (`PrimitiveComponent.SetCollisionEnabled` _mesh "NoCollision")
  (bind (_direction _rate) (`Timeline|タイムライン_0`)
    (:`Update`
      (`MeshComponent.SetScalarParameterValueOnMaterials` (`self.Mesh`) "Rate" _rate))
    (:`Finished`
      (bind _networktype (`self.Select`))
      (switch `/Game/Character/NetworkType` _networktype
        (:`NewEnumerator0`
          _)
        (:`NewEnumerator2`
          _))
      (`self.K2_DestroyActor`))))

(fn `DethAnimetionStart`
  (if (`self.IsFarAttackFlg`)
    (`self.PlayAnimMontage` (`self.DeathMontage_fly`))
    (else
      (`self.PlayAnimMontage` (`self.DeathMontage`)))))

(fn `UserConstructionScript`
  (`parent.UserConstructionScript`))