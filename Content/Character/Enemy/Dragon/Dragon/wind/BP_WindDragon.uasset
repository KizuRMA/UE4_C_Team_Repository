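; Wind dragon enemy character, a child Blueprint that adds its materials, breath attack and death visuals.
; BeginPlay animates mesh opacity, then swaps to the green material.
; Fire spawns a wind breath attached to the breath socket, only for Local or Owner network types, which also gate destruction after the down animation's Rate material timeline.
; Death picks a flying or standard montage from the far-attack flag.
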(event `self.ReceiveBeginPlay`
  (`parent.ReceiveBeginPlay`)
  (bind (_direction _opacity) (`Timeline|タイムライン_1`)
    (:`Update`
      (`MeshComponent.SetScalarParameterValueOnMaterials` (`self.Mesh`) "opacity" _opacity))
    (:`Finished`
      (`PrimitiveComponent.SetMaterial` (`self.Mesh`) 0 "/Game/FourEvilDragonsHP/Materials/DragonTheTerrorBringer/GreenMat_Inst.GreenMat_Inst"))))

(event `Fire`
  (bind _networktype (`self.Select`))
  (switch `/Game/Character/NetworkType` _networktype
    (:`NewEnumerator0`
      _)
    (:`NewEnumerator2`
      _))
  (bind _returnvalue (`|SpawnActorFromClass` "/Game/Character/Magic/BP_Magic/BP_DragonWindBreath.BP_DragonWindBreath_C" (`KismetMathLibrary.MakeTransform` (`SceneComponent.GetSocketLocation` (`self.Mesh`) "breath") (struct :`Yaw` -90.0)) "Undefined" "OverrideRootScale" self "DragonWind" 0 self))
  (`self.K2_AttachToComponent` _returnvalue (`self.Mesh`) "breath" "SnapToTarget" "KeepRelative" "KeepRelative" true))

(event `Animetion_Down`
  (bind _mesh (`self.Mesh`))
  (`PrimitiveComponent.SetCastShadow` _mesh false)
  (`PrimitiveComponent.SetCollisionEnabled` _mesh "NoCollision")
  (bind (_direction _rate) (`Timeline|タイムライン_0`)
    (:`Update`
      (`MeshComponent.SetScalarParameterValueOnMaterials` (`self.Mesh`) "Rate" _rate))
    (:`Finished`
      (bind _networktype (`self.Select`))
      (switch `/Game/Character/NetworkType` _networktype
        (:`NewEnumerator0`
          _)
        (:`NewEnumerator2`
          _))
      (`self.K2_DestroyActor`))))

(fn `DethAnimetionStart`
  (if (`self.IsFarAttackFlg`)
    (`self.PlayAnimMontage` (`self.DeathMontage_fly`))
    (else
      (`self.PlayAnimMontage` (`self.DeathMontage`)))))

(fn `UserConstructionScript`
  (`parent.UserConstructionScript`))