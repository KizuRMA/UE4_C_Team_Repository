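; BP_EnemySpawnPoint_new is an enemy spawn point that periodically tops up enemies around itself, on a tick interval set at BeginPlay.
; When connected to a Strix room server, only the room owner that also owns the replicator runs the check; unconnected, it runs directly.
; While actors overlapping EnemyCheckSphere number below PopLimit, it spawns a random PopEnemyList class at a random reachable point within Sphere's radius, with debug prints.
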(event `self.ReceiveBeginPlay`
  (`self.SetActorTickInterval` (`self.tickInterval`)))

(event `self.ReceiveTick`
  (params (DeltaSeconds :type "Float (single-precision)"))
  (bind _returnvalue (`StrixBlueprintFunctionLibrary.IsRoomServerConnected` 0))
  (if _returnvalue
    (bind _returnvalue_2 (`StrixBlueprintFunctionLibrary.IsRoomOwner` 0))
    (if (and _returnvalue_2 (`StrixReplicatorComponent.GetIsOwner` (`self.StrixReplicator`)))
      (bind _poppossible (`self.EnemyCheck` :!label _label)
        (:`NewParam2`
          (if _poppossible
            (`self.PopEnemy`)
            (`KismetSystemLibrary.PrintString` "Spawn")))))
    (else
      (goto _label))))

(fn `PopEnemy`
  (`|SpawnActorFromClass` (`KismetArrayLibrary.Array_Random` (`self.PopEnemyList`)) (`KismetMathLibrary.MakeTransform` (`NavigationSystemV1.K2_GetRandomReachablePointInRadius` (`self.K2_GetActorLocation`) (`SphereComponent.SphereRadius` (`self.Sphere`)) null null)) "Undefined" "OverrideRootScale" null null))

(fn `UserConstructionScript`)