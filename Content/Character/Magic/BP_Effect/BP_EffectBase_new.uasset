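; Base actor for magic effects that plays a configurable particle template and manages its own lifetime alongside a Parent object.
; On BeginPlay it assigns the template to its particle component.
; When the particles finish it destroys itself, first setting the Parent's delete flag if auto-destroy is enabled.
; Unless marked as a hit effect, it checks every Tick and destroys itself once the Parent becomes invalid.
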(event `self.ReceiveBeginPlay`
  (`ParticleSystemComponent.SetTemplate` (`self.ParticleSystem`) (`self.Particle`)))

(event `self.ParticleSystem.OnSystemFinished`
  (params (PSystem :type "ParticleSystemComponent Object Reference"))
  (`|ExecutionSequence`
    (:`then_0`
      (if (`self.AutoDestry`)
        (bind _parent (`self.Parent`)
          (:`then`
            (set `/Game/Character/Magic/BP_Magic/BP_MagicBase_new.DeleteFlg` true _parent))
          (:`else`))))
    (:`then_1`
      (`self.K2_DestroyActor`))))

(event `self.ReceiveTick`
  (params (DeltaSeconds :type "Float (single-precision)"))
  (if (not (`self.hitEffect`))
    (`self.Parent`
      (:`then`)
      (:`else`
        (`self.K2_DestroyActor`)))))

(fn `UserConstructionScript`)