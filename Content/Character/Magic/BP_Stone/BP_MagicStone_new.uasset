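; BP_MagicStone_new is a magic stone actor that pops upward with a random sideways velocity when spawned.
; BeginPlay builds a BP_MagicInfo_2 object from the data table row matching its configured name, then launches through ProjectileMovement.
; Tick reapplies that info's mesh every frame, or destroys the actor if the info's name is None.
; SetMagicInfoAndVisual replaces the info and updates the mesh immediately.
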(event `self.ReceiveBeginPlay`
  ;[1 1 1] 初期化処理
  (`self.Setup Magic Info` (`.Name_17_63CCF482466D9911C84E998894370AB7` (break `/Game/Character/Magic/Data/MagicStoneData` (`self.datas`))))
  (`self.Projectile Random Velocity`))

(event `self.ReceiveTick`
  (params (DeltaSeconds :type "Float (single-precision)"))
  (bind (_magic_info_difine_name _magic_info_difine_id _magic_info_difine_mesh) (break `/Game/Character/Magic/Data/MagicStoneData` (`/Game/Character/Cleric/WBP/Inventry/BP_MagicInfo_2.Magic Info Difine` (`self.magicStoneInfo`))))
  ;[1 1 1] 更新処理
  (if (!= "None" _magic_info_difine_name)
    (`StaticMeshComponent.SetStaticMesh` (`self.StaticMesh`) _magic_info_difine_mesh)
    (else
      (`self.K2_DestroyActor`))))

(event `Set Magic Info And Visual`
  (params (`Magic Info` :type "/Game/Character/Cleric/WBP/Inventry/BP_MagicInfo_2 Object Reference"))
  ;[1 1 1] 魔石の情報を変更する処理
  (bind _output_get (set `self.magicStoneInfo` `Magic Info`))
  (bind (_magic_info_difine_name _magic_info_difine_id _magic_info_difine_mesh) (break `/Game/Character/Magic/Data/MagicStoneData` (`/Game/Character/Cleric/WBP/Inventry/BP_MagicInfo_2.Magic Info Difine` _output_get)))
  (`StaticMeshComponent.SetStaticMesh` (`self.StaticMesh`) _magic_info_difine_mesh))

(event `Projectile Random Velocity`
  ;[1 1 1] プロジェクタイルの移動方向をランダム化
  (`ProjectileMovementComponent.SetVelocityInLocalSpace` (`self.ProjectileMovement`) (`KismetMathLibrary.MakeVector` (* (`KismetMathLibrary.RandomFloatInRange` -1.0 1.0) 250.0) (* (`KismetMathLibrary.RandomFloatInRange` -1.0 1.0) 250.0) 500.0)))

(fn `DataSetup`
  (bind (_magic_info_difine_name _magic_info_difine_id _magic_info_difine_mesh) (break `/Game/Character/Magic/Data/MagicStoneData` (`/Game/Character/Cleric/WBP/Inventry/BP_MagicInfo_2.Magic Info Difine` (`self.magicStoneInfo`))))
  (`StaticMeshComponent.SetStaticMesh` (`self.StaticMesh`) _magic_info_difine_mesh))

(fn `Setup Magic Info`
  (params (TypeName :type Name))
  (bind _returnvalue (`|GenericCreateObject` "/Game/Character/Cleric/WBP/Inventry/BP_MagicInfo_2.BP_MagicInfo_2_C" self))
  (bind _returnvalue_2 (`|GetDataTableRow` "/Game/Character/Magic/Data/MagicStoneDaataTable.MagicStoneDaataTable" TypeName)
    (:`then`
      (set `/Game/Character/Cleric/WBP/Inventry/BP_MagicInfo_2.Magic Info Difine` _returnvalue_2 _returnvalue)
      (set `self.magicStoneInfo` _returnvalue))))

(fn `UserConstructionScript`)