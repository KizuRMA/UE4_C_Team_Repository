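; BP_RockBall_new is a short-lived rock ball magic actor that builds on a parent Blueprint or class.
; On BeginPlay it runs the parent logic, then destroys itself after a brief fixed delay.
; CreateHitEffect spawns BP_RockHitEffect at the actor's transform regardless of collisions, with no caller in this graph.
; The overlap and tick events are disabled placeholders, and construction only calls the parent.
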(event `self.ReceiveBeginPlay`
  (`parent.ReceiveBeginPlay`)
  (`KismetSystemLibrary.Delay` 2.0)
  (`self.K2_DestroyActor`))

(fn `CreateHitEffect`
  (`|SpawnActorFromClass` "/Game/Character/Magic/BP_Magic/Hit/BP_RockHitEffect.BP_RockHitEffect_C" (`self.GetTransform`) "AlwaysSpawn" "OverrideRootScale" null null))

(fn `UserConstructionScript`
  (`parent.UserConstructionScript`))