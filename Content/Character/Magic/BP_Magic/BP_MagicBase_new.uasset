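; Base magic spell actor that spawns effects and damages characters, configured by its Spell row in DT_MagicTable.
; Init either launches it toward the target or places it on the ground there.
; Begin-overlap, plus per-tick checks on overlapping enemies, feed Attack, which applies elemental damage, hit effects and optional destroy-on-hit.
; Events branch through a Local/Owner/Client select macro, running offline directly or via Strix RPCs when connected to a room.
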(event `Attack`
  (params (DamagPoint :type Integer))
  ;[1 1 1] 与ダメージ時
  (bind _isroomowner (`self.Select_macro`)
    (:`LocalActor`
      (`self.AttackFunction_Local` DamagPoint))
    (:`OwnerActor`
      (`StrixBlueprintFunctionLibrary.SendRpcToAll` null "AttackFunction_Owner_Strix" (`|MakeArray` (`StrixBlueprintFunctionLibrary.Conv_IntToStrixRelayArg` DamagPoint) (`StrixBlueprintFunctionLibrary.Conv_BoolToStrixRelayArg` _isroomowner)) :!label _label))
    (:`ClientActor`
      (goto _label))))

(event `self.ReceiveBeginPlay`
  ;[1 1 1] 開始時
  (`self.Select_macro`
    (:`LocalActor`
      (`self.Begin_Local`)
      (`self.Create Effect` (`self.Spell`)))))

(event `self.StrixReplicator.OnSyncBegin`
  ;[1 1 1] 開始時
  (`self.SetStrixFunction`)
  (bind _isroomowner (`self.Select_macro`)
    (:`OwnerActor`
      (`self.Begin_Owner_Strix` _isroomowner)
      (`StrixBlueprintFunctionLibrary.SendRpcToAll` null "Create Effect" (`|MakeArray` (`StrixBlueprintFunctionLibrary.Conv_StringToStrixRelayArg` (`self.Spell`)))))))

(event `self.ReceiveActorEndOverlap`
  (params (OtherActor :type "Actor Object Reference"))
  ;[1 1 1] 重なり終わった時
  (bind _isroomowner (`self.Select_macro`)
    (:`LocalActor`
      (`self.EndOverlap_Local` OtherActor))
    (:`OwnerActor`
      (`self.EndOverlap_Owner_Strix` OtherActor _isroomowner :!label _label_2))
    (:`ClientActor`
      (goto _label_2))))

(event `self.ReceiveHit`
  (params (MyComp :type "PrimitiveComponent Object Reference") (Other :type "Actor Object Reference") (OtherComp :type "PrimitiveComponent Object Reference") (bSelfMoved :type Boolean) (HitLocation :type "Vector Structure") (HitNormal :type "Vector Structure") (NormalImpulse :type "Vector Structure") (Hit :type "HitResult Structure (by ref)"))
  ;[1 1 1] 接触時
  (`KismetSystemLibrary.PrintString` (`KismetSystemLibrary.GetDisplayName` Other))
  (bind _isroomowner (`self.Select_macro`)
    (:`LocalActor`
      (`self.Hit_Local` Other HitLocation))
    (:`OwnerActor`
      (`self.Hit_Owner_Strix` Other HitLocation _isroomowner))))

(event `self.ReceiveActorBeginOverlap`
  (params (OtherActor :type "Actor Object Reference"))
  ;[1 1 1] 重なり始めた時
  (`KismetSystemLibrary.PrintString` (`KismetSystemLibrary.GetDisplayName` OtherActor))
  (bind _isroomowner (`self.Select_macro`)
    (:`LocalActor`
      (`self.BeginOverlap_Local` OtherActor))
    (:`OwnerActor`
      (`self.BeginOverlap_Owner_Strix` OtherActor _isroomowner :!label _label_3))
    (:`ClientActor`
      (goto _label_3))))

(event `self.ReceiveTick`
  (params (DeltaSeconds :type "Float (single-precision)"))
  ;[1 1 1] 定期実行
  (bind _isroomowner (`self.Select_macro`)
    (:`LocalActor`
      (`self.Tick_Local` DeltaSeconds))
    (:`OwnerActor`
      (`self.Tick_Owner_Strix` _isroomowner DeltaSeconds :!label _label_4))
    (:`ClientActor`
      (goto _label_4))))

(fn `AttackFunction_Client_Strix`
  (params (Player :type "Actor Object Reference") (DamagePoint :type Integer) (IsRoomOwner :type Boolean)))

(fn `AttackFunction_Local`
  (params (DamagePoint :type Integer))
  (if (`self.ActorHasTag` (`self.hitActor`) "Character")
    (bind _asbp_character (cast `/Game/Character/BP_Character` (`self.hitActor`)))
    (`|ExecutionSequence`
      (:`then_0`
        ;[1 1 1] スコア加算処理で使用する
        (bind _asbp_enemy_base (cast `/Game/Character/Enemy/Base/BP_EnemyBase` (`self.hitActor`)))
        (set `/Game/Character/Enemy/Base/BP_EnemyBase.Actor` (`self.Instigator`) _asbp_enemy_base))
      (:`then_1`
        (bind _returnvalue (`|GetDataTableRow` "/Game/DataTable/DT_MagicTable.DT_MagicTable" (`KismetStringLibrary.Conv_StringToName` (`self.Spell`)))
          (:`then`
            (`/Game/Character/BP_Character.Damaged` _asbp_character DamagePoint (`self.RoomMenberID`) 0 (`self.K2_GetActorLocation`) (`.ElementType_40_992E047C469D744E793B13ACF7043F1F` (break `/Game/Character/Magic/Data/MagicData` _returnvalue)))
            (`self.Delete`)))))))

(fn `AttackFunction_Owner_Strix`
  (params (DamagePoint :type Integer) (IsRoomOwner :type Boolean))
  (bind _hitactor (`self.hitActor`)
    (:`then`
      (if (`self.ActorHasTag` _hitactor "Character")
        (`|ExecutionSequence`
          (:`then_0`
            ;[1 1 1] スコア加算処理で使用する
            (bind _asbp_enemy_base (cast `/Game/Character/Enemy/Base/BP_EnemyBase` (`self.hitActor`)))
            (set `/Game/Character/Enemy/Base/BP_EnemyBase.Actor` (`self.Instigator`) _asbp_enemy_base))
          (:`then_1`
            (bind _returnvalue (`|GetDataTableRow` "/Game/DataTable/DT_MagicTable.DT_MagicTable" (`KismetStringLibrary.Conv_StringToName` (`self.Spell`)))
              (:`then`
                (`StrixBlueprintFunctionLibrary.SendRpcToObjectOwner` (`self.hitActor`) "Damaged" (`|MakeArray` (`StrixBlueprintFunctionLibrary.Conv_IntToStrixRelayArg` DamagePoint) (`StrixBlueprintFunctionLibrary.Conv_IntToStrixRelayArg` (`self.RoomMenberID`)) (`StrixBlueprintFunctionLibrary.Conv_IntToStrixRelayArg` (`self.PlayerControllerID`)) (`StrixBlueprintFunctionLibrary.Conv_VectorToStrixRelayArg` (`self.K2_GetActorLocation`)) (`StrixBlueprintFunctionLibrary.Conv_ByteToStrixRelayArg` (`.ElementType_40_992E047C469D744E793B13ACF7043F1F` (break `/Game/Character/Magic/Data/MagicData` _returnvalue)))))
                (`StrixBlueprintFunctionLibrary.SendRpcToAll` null "CreateHitEffect")
                (bind _returnvalue_2 (`|GetDataTableRow` "/Game/DataTable/DT_MagicTable.DT_MagicTable" (`KismetStringLibrary.Conv_StringToName` (`self.Spell`)))
                  (:`then`
                    (if (`.OneHitDestroy_31_7567D54E4E985CCA39605B9C9FDB3050` (break `/Game/Character/Magic/Data/MagicData` _returnvalue_2))
                      (`self.Select_macro`
                        (:`OwnerActor`
                          (`self.K2_DestroyActor`))))))))))))
    (:`else`)))

(fn `Begin_Client_Strix`
  (params (IsRoomOwner :type Boolean)))

(fn `Begin_Local`)

(fn `Begin_Owner_Strix`
  (params (IsRoomOwner :type Boolean)))

(fn `BeginOverlap_Client_Strix`
  (params (HitActor :type "Actor Object Reference") (IsRoomOwner :type Boolean)))

(fn `BeginOverlap_Local`
  (params (HitActor :type "Actor Object Reference"))
  (if (`self.ActorHasTag` HitActor "Character")
    (set `self.hitActor` HitActor)
    (bind _returnvalue (`|GetDataTableRow` "/Game/DataTable/DT_MagicTable.DT_MagicTable" (`KismetStringLibrary.Conv_StringToName` (`self.Spell`)))
      (:`then`
        (`self.Attack` (`.Damage_5_178004FC45F21871F5B4DEA0E6DDB2A6` (break `/Game/Character/Magic/Data/MagicData` _returnvalue)))))
    (else
      (`self.Delete`))))

(fn `BeginOverlap_Owner_Strix`
  (params (HitActor :type "Actor Object Reference") (IsRoomOwner :type Boolean))
  (if (`self.ActorHasTag` HitActor "Character")
    (set `self.hitActor` HitActor)
    (bind _returnvalue (`|GetDataTableRow` "/Game/DataTable/DT_MagicTable.DT_MagicTable" (`KismetStringLibrary.Conv_StringToName` (`self.Spell`)))
      (:`then`
        (`self.Attack` (`.Damage_5_178004FC45F21871F5B4DEA0E6DDB2A6` (break `/Game/Character/Magic/Data/MagicData` _returnvalue)))))
    (else
      (`StrixBlueprintFunctionLibrary.SendRpcToAll` null "CreateHitEffect")
      (bind _returnvalue_2 (`|GetDataTableRow` "/Game/DataTable/DT_MagicTable.DT_MagicTable" (`KismetStringLibrary.Conv_StringToName` (`self.Spell`)))
        (:`then`
          (if (`.OneHitDestroy_31_7567D54E4E985CCA39605B9C9FDB3050` (break `/Game/Character/Magic/Data/MagicData` _returnvalue_2))
            (`self.Select_macro`
              (:`OwnerActor`
                (`self.K2_DestroyActor`)))))))))

(fn `Create Effect`
  (params (spell :type String))
  (`|ExecutionSequence`
    (:`then_0`
      (bind _returnvalue (`|GetDataTableRow` "/Game/DataTable/DT_MagicTable.DT_MagicTable" (`KismetStringLibrary.Conv_StringToName` spell))
        (:`then`
          (bind (_magicclass _damage _effect _hiteffect _magicspawntype _effectenddestroy) (break `/Game/Character/Magic/Data/MagicData` _returnvalue))
          (if (not (== _magicclass "BP_MagicBase_new_C"))
            (`/Engine/EditorBlueprintResources/StandardMacros.IsValid` _effect
              (:`Is Valid`
                (bind _returnvalue_2 (`|SpawnActorFromClass` "/Game/Character/Magic/BP_Effect/BP_EffectBase_new.BP_EffectBase_new_C" (`self.GetTransform`) "AlwaysSpawn" "OverrideRootScale" null _effectenddestroy self _effect false null))
                (`self.K2_AttachToActor` _returnvalue_2 self "None" "SnapToTarget" "SnapToTarget" "KeepWorld" true)))))))
    (:`then_1`
      (`self.Select_macro`
        (:`LocalActor`
          _)
        (:`OwnerActor`
          _)
        (:`ClientActor`
          _))
      (set `self.Spell` spell))))

(fn `CreateHitEffect`
  (bind _returnvalue (`|GetDataTableRow` "/Game/DataTable/DT_MagicTable.DT_MagicTable" (`KismetStringLibrary.Conv_StringToName` (`self.Spell`)))
    (:`then`
      (bind (_magicclass _damage _effect _hiteffect) (break `/Game/Character/Magic/Data/MagicData` _returnvalue))
      (`/Engine/EditorBlueprintResources/StandardMacros.IsValid` _hiteffect
        (:`Is Valid`
          (`|SpawnActorFromClass` "/Game/Character/Magic/BP_Effect/BP_EffectBase_new.BP_EffectBase_new_C" (`self.GetTransform`) "AlwaysSpawn" "OverrideRootScale" null true null _hiteffect true null))))))

(fn `Delete`
  (`self.CreateHitEffect`)
  (bind _returnvalue (`|GetDataTableRow` "/Game/DataTable/DT_MagicTable.DT_MagicTable" (`KismetStringLibrary.Conv_StringToName` (`self.Spell`)))
    (:`then`
      (if (`.OneHitDestroy_31_7567D54E4E985CCA39605B9C9FDB3050` (break `/Game/Character/Magic/Data/MagicData` _returnvalue))
        (`self.K2_DestroyActor`)))))

(fn `EndOverlap_Client_Strix`
  (params (HitActor :type "Actor Object Reference") (IsRoomOwner :type Boolean)))

(fn `EndOverlap_Local`
  (params (HitActor :type "Actor Object Reference")))

(fn `EndOverlap_Owner_Strix`
  (params (HitActor :type "Actor Object Reference") (IsRoomOwner :type Boolean)))

(fn `Hit_Client_Strix`
  (params (HitActor :type "Actor Object Reference") (HitLocation :type "Vector Structure") (IsRoomOwner :type Boolean)))

(fn `Hit_Local`
  (params (HitActor :type "Actor Object Reference") (HitLocation :type "Vector Structure")))

(fn `Hit_Owner_Strix`
  (params (HitActor :type "Actor Object Reference") (HitLocation :type "Vector Structure") (IsRoomOwner :type Boolean)))

(fn `Init`
  (params (TargetPoint :type "Vector Structure") (SpawnPoint :type "Vector Structure"))
  (bind _returnvalue (- TargetPoint SpawnPoint))
  (bind _returnvalue_2 (`|GetDataTableRow` "/Game/DataTable/DT_MagicTable.DT_MagicTable" (`KismetStringLibrary.Conv_StringToName` (`self.Spell`)))
    (:`then`
      (switch `/Game/Character/Magic/Data/MagicSpawnType` (`.MagicSpawnType_23_FD130D534C2A12A114C0C7AF50C824AB` (break `/Game/Character/Magic/Data/MagicData` _returnvalue_2))
        (:`NewEnumerator0`
          ;[1 1 1] 出現位置設定
          (`self.K2_SetActorTransform` (`KismetMathLibrary.MakeTransform` SpawnPoint (`KismetMathLibrary.MakeRotFromZ` _returnvalue)))
          ;[1 1 1] Projectailを新しいTransformに合わせる
          (set `MovementComponent.Velocity` (* (`KismetMathLibrary.Normal` _returnvalue) 500.0) (`self.ProjectileMovement`)))
        (:`NewEnumerator1`
          ;[1 1 1] 出現位置を設定
          (bind _outhit (`KismetSystemLibrary.LineTraceSingle` :`Start` TargetPoint :`End` (- TargetPoint (0.0 0.0 5000.0)) :`TraceChannel` "TraceTypeQuery3" :`DrawDebugType` "ForOneFrame"))
          (bind (_bblockinghit _binitialoverlap _time _distance _location) (`GameplayStatics.BreakHitResult` _outhit))
          (if _bblockinghit
            (`self.K2_SetActorLocation` _location)
            (else
              (`self.K2_SetActorLocation` TargetPoint))))))))

(fn `Select`
  (returns (NetWorkType :type "/Game/Character/NetworkType Enum") (IsRoomOwner :type Boolean))
  (`|ExecutionSequence`
    (:`then_0`
      (bind _returnvalue (`StrixBlueprintFunctionLibrary.IsRoomServerConnected` 0))
      (if (not _returnvalue)
        (return "NewEnumerator0" false)))
    (:`then_1`
      (if (`StrixReplicatorComponent.GetIsOwner` (`self.StrixReplicator`))
        (bind _returnvalue_2 (`StrixBlueprintFunctionLibrary.IsRoomOwner` 0))
        (return "NewEnumerator2" _returnvalue_2)
        (else
          (bind _returnvalue_3 (`StrixBlueprintFunctionLibrary.IsRoomOwner` 0))
          (return "NewEnumerator3" _returnvalue_3))))))

(fn `SetStrixFunction`
  (`StrixBlueprintFunctionLibrary.RegisterStrixRpc` null "Create Effect")
  (`StrixBlueprintFunctionLibrary.RegisterStrixRpc` null "AttackFunction_Owner_Strix")
  (`StrixBlueprintFunctionLibrary.RegisterStrixRpc` null "Attack")
  (`StrixBlueprintFunctionLibrary.RegisterStrixRpc` null "CreateHitEffect"))

(fn `Tick_Client_Strix`
  (params (IsRoomOwner :type Boolean) (DeltaSecondes :type "Float (double-precision)")))

(fn `Tick_Local`
  (params (DeltaSecondes :type "Float (double-precision)"))
  (`|ExecutionSequence`
    (:`then_0`
      (for _array_element (`self.GetOverlappingActors` "/Game/Character/BP_Character.BP_Character_C")
        (set `self.hitActor` _array_element)
        (if (`self.ActorHasTag` _array_element "Enemy")
          (cast `/Game/Character/Enemy/Base/BP_EnemyBase` _array_element)
          (bind _returnvalue (`|GetDataTableRow` "/Game/DataTable/DT_MagicTable.DT_MagicTable" (`KismetStringLibrary.Conv_StringToName` (`self.Spell`)))
            (:`then`
              (`self.Attack` (`.Damage_5_178004FC45F21871F5B4DEA0E6DDB2A6` (break `/Game/Character/Magic/Data/MagicData` _returnvalue))))))))
    (:`then_1`
      (if (`self.DeleteFlg`)
        (`self.K2_DestroyActor`)))))

(fn `Tick_Owner_Strix`
  (params (IsRoomOwner :type Boolean) (DeltaSecondes :type "Float (double-precision)"))
  (`|ExecutionSequence`
    (:`then_0`
      (if (`self.DeleteFlg`)
        (`self.K2_DestroyActor`)))
    (:`then_1`
      (for _array_element (`self.GetOverlappingActors` "/Game/Character/BP_Character.BP_Character_C")
        (set `self.hitActor` _array_element)
        (if (`self.ActorHasTag` _array_element "Enemy")
          (cast `/Game/Character/Enemy/Base/BP_EnemyBase` _array_element)
          (bind _returnvalue (`|GetDataTableRow` "/Game/DataTable/DT_MagicTable.DT_MagicTable" (`KismetStringLibrary.Conv_StringToName` (`self.Spell`)))
            (:`then`
              (`self.Attack` (`.Damage_5_178004FC45F21871F5B4DEA0E6DDB2A6` (break `/Game/Character/Magic/Data/MagicData` _returnvalue))))))))))

(fn `UserConstructionScript`)