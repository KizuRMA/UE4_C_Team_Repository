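; Thunderbolt magic Blueprint that provides the effect and sound for the spell's hit.
; CreateHitThunderEffect looks up the Spell's row in DT_MagicTable and spawns an auto-destroying BP_EffectBase_new with the row's hit particle, falling back to the HitEffect class if none is valid.
; It then plays the row's hit sound, if set, at the actor's location with attenuation.
; The construction script only calls the parent.
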(fn `Create HitThunder Effect`
  (bind _returnvalue (`self.GetTransform`))
  (bind _returnvalue_2 (`|GetDataTableRow` "/Game/DataTable/DT_MagicTable.DT_MagicTable" (`KismetStringLibrary.Conv_StringToName` (`self.Spell`)))
    (:`then`
      (`|ExecutionSequence`
        (:`then_0`
          (bind (_magicclass _damage _effect _hiteffect _magicspawntype _effectenddestroy _onehitdestroy _elementtype _createsound _hitsound) (break `/Game/Character/Magic/Data/MagicData` _returnvalue_2))
          (`/Engine/EditorBlueprintResources/StandardMacros.IsValid` _hiteffect
            (:`Is Valid`
              (`|SpawnActorFromClass` "/Game/Character/Magic/BP_Effect/BP_EffectBase_new.BP_EffectBase_new_C" _returnvalue "AlwaysSpawn" "OverrideRootScale" null true null _hiteffect true null))
            (:`Is Not Valid`
              (`|SpawnActorFromClass` (`self.hitEffect`) _returnvalue "AlwaysSpawn" "OverrideRootScale" null null))))
        (:`then_1`
          ;[1 1 1] 衝突時の音を再生
          (`/Engine/EditorBlueprintResources/StandardMacros.IsValid` _hitsound
            (:`Is Valid`
              (`GameplayStatics.PlaySoundAtLocation` _hitsound (`self.K2_GetActorLocation`) (struct) 1.0 1.0 0.0 "/Game/Sound/SoundAttenuation.SoundAttenuation" null null))))))))

(fn `UserConstructionScript`
  (`parent.UserConstructionScript`))