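; Base character Blueprint for Strix-networked play, with mostly empty hook functions for begin, damage, attack, death, hit and overlap.
; A Select macro routes events to Local, Owner or Client variants based on room connection and replicator ownership.
; Owners broadcast damage, attack and death via Strix RPCs registered on sync begin, with death following an HP check.
; DamageCalc scales damage by elemental affinity, and OnRep HP feeds an empty update hook.
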(event `self.ReceiveBeginPlay`
  ;[1 1 1] 開始時
  (`self.Select_macro`
    (:`LocalActor`
      (`self.BeginFunction_Local`))))

(event `self.StrixReplicator.OnSyncBegin`
  ;[1 1 1] 開始時
  (`self.SetStrixFunction`)
  (bind _isroomowner (`self.Select_macro`)
    (:`OwnerActor`
      (`self.BeginFunction_Owner_Strix` _isroomowner))
    (:`ClientActor`
      (`self.BeginFunction_Client_Strix` _isroomowner))))

(event `Attack`
  (params (playerControllerID :type Integer) (DamagPoint :type Integer))
  ;[1 1 1] 与ダメージ時
  (bind _isroomowner (`self.Select_macro`)
    (:`LocalActor`
      (`self.AttackFunction_Local` playerControllerID DamagPoint))
    (:`OwnerActor`
      (`StrixBlueprintFunctionLibrary.SendRpcToAll` null "AttackFunction_Owner_Strix" (`|MakeArray` (`StrixBlueprintFunctionLibrary.Conv_IntToStrixRelayArg` playerControllerID) (`StrixBlueprintFunctionLibrary.Conv_IntToStrixRelayArg` DamagPoint) (`StrixBlueprintFunctionLibrary.Conv_BoolToStrixRelayArg` _isroomowner))))))

(event `Damaged`
  (params (DamagePoint :type Integer) (RoomMenberID :type Integer) (playerControllerID :type Integer) (Vector :type "Vector Structure") (Element :type "/Game/Character/Magic/Data/ElementType Enum" :default "NewEnumerator0"))
  ;[1 1 1] 被ダメージ時
  (bind _isroomowner (`self.Select_macro`)
    (:`LocalActor`
      (`self.DamageFunction_Local` DamagePoint playerControllerID Vector Element)
      (`KismetSystemLibrary.Delay` 0.1)
      (if (<= (`self.HP`) 0)
        (`self.DeathFunction_Local` playerControllerID)))
    (:`OwnerActor`
      (`KismetSystemLibrary.Delay` 0.1)
      (`StrixBlueprintFunctionLibrary.SendRpcToAll` null "DamageFunction_Owner_Strix" (`|MakeArray` (`StrixBlueprintFunctionLibrary.Conv_IntToStrixRelayArg` DamagePoint) (`StrixBlueprintFunctionLibrary.Conv_IntToStrixRelayArg` RoomMenberID) (`StrixBlueprintFunctionLibrary.Conv_BoolToStrixRelayArg` _isroomowner) (`StrixBlueprintFunctionLibrary.Conv_VectorToStrixRelayArg` Vector) (`StrixBlueprintFunctionLibrary.Conv_ByteToStrixRelayArg` Element)))
      (`KismetSystemLibrary.Delay` 0.1)
      (if (<= (`self.HP`) 0)
        (`StrixBlueprintFunctionLibrary.SendRpcToAll` null "DeathFunction_Owner_Strix" (`|MakeArray` (`StrixBlueprintFunctionLibrary.Conv_IntToStrixRelayArg` RoomMenberID)))))))

(event `self.ReceiveHit`
  (params (MyComp :type "PrimitiveComponent Object Reference") (Other :type "Actor Object Reference") (OtherComp :type "PrimitiveComponent Object Reference") (bSelfMoved :type Boolean) (HitLocation :type "Vector Structure") (HitNormal :type "Vector Structure") (NormalImpulse :type "Vector Structure") (Hit :type "HitResult Structure (by ref)"))
  ;[1 1 1] 接触時
  (bind _isroomowner (`self.Select_macro`)
    (:`LocalActor`
      (`self.HitFunction_Local` Other HitLocation))
    (:`OwnerActor`
      (`self.HitFunction_Owner_Strix` Other HitLocation _isroomowner :!label _label))
    (:`ClientActor`
      (goto _label))))

(event `self.ReceiveActorEndOverlap`
  (params (OtherActor :type "Actor Object Reference"))
  ;[1 1 1] 重なり終わった時
  (bind _isroomowner (`self.Select_macro`)
    (:`LocalActor`
      (`self.EndOverlapFunction_Local` OtherActor))
    (:`OwnerActor`
      (`self.EndOverlapFunction_Owner_Strix` OtherActor _isroomowner :!label _label_2))
    (:`ClientActor`
      (goto _label_2))))

(event `self.ReceiveActorBeginOverlap`
  (params (OtherActor :type "Actor Object Reference"))
  ;[1 1 1] 重なり始めた時
  (bind _isroomowner (`self.Select_macro`)
    (:`LocalActor`
      (`self.BeginOverlapFunction_Local` OtherActor))
    (:`OwnerActor`
      (`self.BeginOverlapFunction_Owner_Strix` OtherActor _isroomowner :!label _label_3))
    (:`ClientActor`
      (goto _label_3))))

(fn `AttackFunction_Client_Strix`
  (params (playerControllerID :type Integer) (DamagePoint :type Integer) (IsRoomOwner :type Boolean))
  (return))

(fn `AttackFunction_Local`
  (params (playerControllerID :type Integer) (DamagePoint :type Integer))
  (return))

(fn `AttackFunction_Owner_Strix`
  (params (playerControllerID :type Integer) (DamagePoint :type Integer) (IsRoomOwner :type Boolean))
  (return))

(fn `BeginFunction_Client_Strix`
  (params (IsRoomOwner :type Boolean)))

(fn `BeginFunction_Local`)

(fn `BeginFunction_Owner_Strix`
  (params (IsRoomOwner :type Boolean)))

(fn `BeginOverlapFunction_Client_Strix`
  (params (HitActor :type "Actor Object Reference") (IsRoomOwner :type Boolean)))

(fn `BeginOverlapFunction_Local`
  (params (HitActor :type "Actor Object Reference")))

(fn `BeginOverlapFunction_Owner_Strix`
  (params (HitActor :type "Actor Object Reference") (IsRoomOwner :type Boolean)))

(fn `DamageCalc`
  (params (Damage :type Integer) (Element :type "/Game/Character/Magic/Data/ElementType Enum" :default "NewEnumerator0"))
  (returns (HP :type Integer) (CalcDamage :type Integer) (Compatibility :type "/Game/Character/Magic/Data/ElementIndex Enum"))
  (bind (_value _elementvalue) (`self.ElementDamage` Element))
  (bind _returnvalue (`KismetMathLibrary.FTrunc` (* Damage _value)))
  (bind _output_get (set `self.HP` (- (`self.HP`) _returnvalue)))
  (return _output_get _returnvalue _elementvalue))

(fn `DamageFunction_Client_Strix`
  (params (DamagePoint :type Integer) (RoomMenberID :type Integer) (IsRoomOwner :type Boolean)))

(fn `DamageFunction_Local`
  (params (DamagePoint :type Integer) (playerControllerID :type Integer) (TargetActorLocation :type "Vector Structure") (ElementNumber :type Byte)))

(fn `DamageFunction_Owner_Strix`
  (params (DamagePoint :type Integer) (RoomMenberID :type Integer) (IsRoomOwner :type Boolean) (TargetActorLocation :type "Vector Structure") (ElementType :type Byte)))

(fn `DeathFunction_Client_Strix`
  (params (playerControllerID :type Integer)))

(fn `DeathFunction_Local`
  (params (playerControllerID :type Integer)))

(fn `DeathFunction_Owner_Strix`
  (params (RoomMenberID :type Integer)))

(fn `ElementDamage`
  (params (Element :type "/Game/Character/Magic/Data/ElementType Enum" :default "NewEnumerator0"))
  (returns (value :type "Float (double-precision)") (elementValue :type "/Game/Character/Magic/Data/ElementIndex Enum"))
  (locals (tmp :type "/Game/Character/Magic/Data/ElementIndex Enum" :default "NewEnumerator1"))
  (bind _tmp (`local.tmp`))
  (`|ExecutionSequence`
    (:`then_0`
      (switch `/Game/Character/Magic/Data/ElementType` (`self.MyElementType`)
        (:`NewEnumerator0`
          (switch `/Game/Character/Magic/Data/ElementType` Element
            (:`NewEnumerator1`
              (set `local.tmp` "NewEnumerator0" :!label _label))
            (:`NewEnumerator2`
              (set `local.tmp` "NewEnumerator2"))
            (:`NewEnumerator4`
              (goto _label))))
        (:`NewEnumerator1`
          (switch `/Game/Character/Magic/Data/ElementType` Element
            (:`NewEnumerator0`
              (set `local.tmp` "NewEnumerator2"))
            (:`NewEnumerator2`
              (set `local.tmp` "NewEnumerator0" :!label _label_2))
            (:`NewEnumerator3`
              (goto _label_2))))
        (:`NewEnumerator2`
          (switch `/Game/Character/Magic/Data/ElementType` Element
            (:`NewEnumerator0`
              (set `local.tmp` "NewEnumerator0" :!label _label_3))
            (:`NewEnumerator1`
              (set `local.tmp` "NewEnumerator2"))
            (:`NewEnumerator5`
              (goto _label_3))))))
    (:`then_1`
      (switch `/Game/Character/Magic/Data/ElementIndex` (`local.tmp`)
        (:`NewEnumerator0`
          (return 1.3 _tmp))
        (:`NewEnumerator1`
          (return 1.0 _tmp))
        (:`NewEnumerator2`
          (return 0.7 _tmp))))))

(fn `EndOverlapFunction_Client_Strix`
  (params (HitActor :type "Actor Object Reference") (IsRoomOwner :type Boolean)))

(fn `EndOverlapFunction_Local`
  (params (HitActor :type "Actor Object Reference")))

(fn `EndOverlapFunction_Owner_Strix`
  (params (HitActor :type "Actor Object Reference") (IsRoomOwner :type Boolean)))

(fn `HitFunction_Client_Strix`
  (params (HitActor :type "Actor Object Reference") (HitLocation :type "Vector Structure") (IsRoomOwner :type Boolean)))

(fn `HitFunction_Local`
  (params (HitActor :type "Actor Object Reference") (HitLocation :type "Vector Structure")))

(fn `HitFunction_Owner_Strix`
  (params (HitActor :type "Actor Object Reference") (HitLocation :type "Vector Structure") (IsRoomOwner :type Boolean)))

(fn `HP_Update_Timing`
  (params (hp :type Integer)))

(fn `OnRep_HP`
  (`self.HP_Update_Timing` (`self.HP`)))

(fn `Select`
  (returns (NetWorkType :type "/Game/Character/NetworkType Enum") (IsRoomOwner :type Boolean))
  (`|ExecutionSequence`
    (:`then_0`
      (bind _returnvalue (`StrixBlueprintFunctionLibrary.IsRoomServerConnected` 0))
      (if (not _returnvalue)
        (return "NewEnumerator0" false)))
    (:`then_1`
      (bind _strixreplicator (`self.StrixReplicator`)
        (:`then`
          (if (`StrixReplicatorComponent.GetIsOwner` _strixreplicator)
            (bind _returnvalue_2 (`StrixBlueprintFunctionLibrary.IsRoomOwner` 0))
            (return "NewEnumerator2" _returnvalue_2)
            (else
              (bind _returnvalue_3 (`StrixBlueprintFunctionLibrary.IsRoomOwner` 0))
              (return "NewEnumerator3" _returnvalue_3))))
        (:`else`)))))

(fn `SetStrixFunction`
  (`|ExecutionSequence`
    (:`then_0`
      (`StrixBlueprintFunctionLibrary.RegisterStrixRpc` null "AttackFunction_Owner_Strix"))
    (:`then_1`
      (`StrixBlueprintFunctionLibrary.RegisterStrixRpc` null "Damaged")
      (`StrixBlueprintFunctionLibrary.RegisterStrixRpc` null "DamageFunction_Owner_Strix")
      (`StrixBlueprintFunctionLibrary.RegisterStrixRpc` null "DeathFunction_Owner_Strix"))))

(fn `UserConstructionScript`)