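; HighLevelArea is an overlap-driven audio area actor that signals the local player's cleric character when it crosses the area's bounds.
; On both begin and end overlap, it casts to BP_Cleric_new, checks for a Local network type, and calls PAddSoundType with the same enum value.
; BeginPlay caches the level's BP_FieldAudio actor, which the overlap logic does not use.
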(event `self.ReceiveBeginPlay`
  (bind _returnvalue (`GameplayStatics.GetActorOfClass` "/Game/Audio/Blueprint/BP_FieldAudio.BP_FieldAudio_C"))
  (set `self.Field Actor` _returnvalue))

(event `self.ReceiveActorBeginOverlap`
  (params (OtherActor :type "Actor Object Reference"))
  (bind _asbp_cleric_new (cast `/Game/Character/Cleric/BP_Cleric_new` OtherActor))
  (bind _networktype (`/Game/Character/BP_Character.Select` _asbp_cleric_new))
  (switch `/Game/Character/NetworkType` _networktype
    (:`NewEnumerator0`
      (`/Game/Character/Cleric/BP_Cleric_new.P_Add Sound Type` _asbp_cleric_new "NewEnumerator1"))))

(event `self.ReceiveActorEndOverlap`
  (params (OtherActor :type "Actor Object Reference"))
  (bind _asbp_cleric_new (cast `/Game/Character/Cleric/BP_Cleric_new` OtherActor))
  (bind _networktype (`/Game/Character/BP_Character.Select` _asbp_cleric_new))
  (switch `/Game/Character/NetworkType` _networktype
    (:`NewEnumerator0`
      (`/Game/Character/Cleric/BP_Cleric_new.P_Add Sound Type` _asbp_cleric_new "NewEnumerator1"))))

(fn `UserConstructionScript`)