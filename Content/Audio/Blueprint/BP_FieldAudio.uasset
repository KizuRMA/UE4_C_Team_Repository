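; BP_FieldAudio manages field background music, switching between default, slime and dragon tracks according to the enemy types currently registered.
; Add and remove events keep per-type counters, undoing removals below zero, and the highest type index with a positive count selects the next track.
; ChangeBGM debounces requests with a retriggerable delay, then fades out the current track before fading in the next.
; GameStart fades in the default track.
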(event `Game Start`
  (`AudioComponent.FadeIn` (`self.DefaultBGM`) 1.0 (`self.volume`) 0.0 "Linear"))

(event `self.ReceiveBeginPlay`
  (`KismetArrayLibrary.Array_Add` (`self.Bgm Array`) (`self.DefaultBGM`))
  (`KismetArrayLibrary.Array_Add` (`self.Bgm Array`) (`self.SlimeBGM`))
  (`KismetArrayLibrary.Array_Add` (`self.Bgm Array`) (`self.DoragonBGM`))
  (set `self.BgmMaxCount` (`KismetArrayLibrary.Array_LastIndex` (`self.Bgm Array`)))
  (set `self.Now Play Bgm Number` 0)
  (set `self.Next Play Bgm Number` 0))

(event `Change BGM`
  (`KismetSystemLibrary.RetriggerableDelay` 1.0)
  (if (!= (`self.Now Play Bgm Number`) (`self.Next Play Bgm Number`))
    (`AudioComponent.FadeOut` (`|GetArrayItem` (`self.Bgm Array`) (`self.Now Play Bgm Number`)) (`self.Duration`) 0.0 "Linear")
    (`KismetSystemLibrary.RetriggerableDelay` (`self.Duration`))
    (`AudioComponent.FadeIn` (`|GetArrayItem` (`self.Bgm Array`) (`self.Next Play Bgm Number`)) (`self.Duration`) (`self.volume`) 0.0 "Linear")
    (set `self.Now Play Bgm Number` (`self.Next Play Bgm Number`))))

(event `Change Next Play Number`
  (set `self.Next Play Bgm Number` 0)
  (for (_array_element _array_index) (`self.TrackTypes`)
    (if (> _array_element 0)
      (set `self.Next Play Bgm Number` _array_index))))

(event `Add Track Type`
  (params (Type :type Integer))
  (bind _result (`/Engine/EditorBlueprintResources/StandardMacros.IncrementInt` (`|GetArrayItem` (`self.TrackTypes`) Type))
    (:`  `
      (`self.Change Next Play Number`)
      (`self.Change BGM`)
      (`KismetSystemLibrary.PrintString` (`KismetStringLibrary.Concat_StrStr` "現在保存している敵の数：" (`KismetStringLibrary.Conv_IntToString` _result))))))

(event `Remove Track Type`
  (params (Type :type Integer))
  (bind _output (`|GetArrayItem` (`self.TrackTypes`) Type))
  (bind _result (`/Engine/EditorBlueprintResources/StandardMacros.DecrementInt` _output)
    (:`  `
      (if (>= _result 0)
        (`self.Change Next Play Number`)
        (`self.Change BGM`)
        (`KismetSystemLibrary.PrintString` (`KismetStringLibrary.Concat_StrStr` "現在保存している敵の数：" (`KismetStringLibrary.Conv_IntToString` _result)))
        (else
          (`/Engine/EditorBlueprintResources/StandardMacros.IncrementInt` _output))))))

(fn `UserConstructionScript`)