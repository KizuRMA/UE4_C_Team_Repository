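; BP_Order arranges BP_LobbyCleric characters on player starts in the main menu lobby and lights their spots.
; Every Tick it runs Order, which uses Strix replicator ownership to put the locally owned cleric at the first start.
; Other clerics take the first unoccupied of the three remaining starts, tracked in the IsPlayer array.
; That array then switches each slot's spotlight on or off.
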(event `self.ReceiveTick`
  (params (DeltaSeconds :type "Float (single-precision)"))
  (`self.Order`))

(fn `Order`
  (locals (IsPlayer :type "Array of Boolean"))
  (bind _outactors (`GameplayStatics.GetAllActorsOfClass` "/Game/Scene/MainMenu/BP_LobbyCleric.BP_LobbyCleric_C"))
  (for _array_element _outactors
    (if (`StrixReplicatorComponent.GetIsOwner` (`/Game/Scene/MainMenu/BP_LobbyCleric.StrixReplicator` _array_element))
      ;[0 0.922 1] 自機の位置を設定
      (`self.K2_SetActorTransform` _array_element (`self.GetTransform` (`|GetArrayItem` (`self.PlayerStarts`))) false false)
      (`KismetArrayLibrary.Array_Set` (`local.IsPlayer`) 0 true)
      (else
        ;[0.9261 1 0.175] クライアントの位置を設定
        (for _index (range 1 4)
          (if (not (`|GetArrayItem` (`local.IsPlayer`) _index))
            (`self.K2_SetActorTransform` _array_element (`self.GetTransform` (`|GetArrayItem` (`self.PlayerStarts`) _index)) false false)
            (`KismetArrayLibrary.Array_Set` (`local.IsPlayer`) _index true)
            (break))))))
  ;[1 1 1] スポットライトの設定
  (for (_array_element_2 _array_index) (`self.SpotLight`)
    (`/Game/Resouce/Spotlight/BP_Spotlight.LightSwitch` _array_element_2 (`|GetArrayItem` (`local.IsPlayer`) _array_index))))

(fn `UserConstructionScript`)