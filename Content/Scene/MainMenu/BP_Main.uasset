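; BP_Main, under the MainMenu scene folder, overrides ChoosePlayerStart in the manner of a game mode to pick where players spawn.
; The live path returns the first actor tagged "0" for every player, with no empty check.
; An unreachable branch maps the current room member's index to a matching actor tag, falling back to the first PlayerStart.
; BeginPlay, Tick and the construction script are empty.
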(fn `ChoosePlayerStart`
  (params (Player :type "Controller Object Reference"))
  (returns (ReturnValue :type "Actor Object Reference"))
  (bind _outactors (`GameplayStatics.GetAllActorsWithTag` "0"))
  (return (`|GetArrayItem` _outactors)))

(fn `UserConstructionScript`)