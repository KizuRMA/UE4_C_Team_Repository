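; Multiplayer lobby cleric avatar that represents a player in a Strix room, with name tag, per-slot material and ready state.
; On sync, the owning copy opens the menu and registers with the room owner, which relays the roster into each Game Instance, while remote copies claim free tagged spots.
; Play toggles readiness or, for the room owner, starts the level once all are ready.
; Leaving broadcasts removal and refreshes slots.
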(event `self.StrixReplicator.OnSyncBegin`
  (`|ExecutionSequence`
    (:`then_0`
      (`StrixBlueprintFunctionLibrary.RegisterStrixRpc` null "SetMember")
      (`StrixBlueprintFunctionLibrary.RegisterStrixRpc` null "SetOtherMember")
      (`StrixBlueprintFunctionLibrary.RegisterStrixRpc` null "COUNT")
      (`StrixBlueprintFunctionLibrary.RegisterStrixRpc` null "GoToLevel")
      (`StrixBlueprintFunctionLibrary.RegisterStrixRpc` null "Remove"))
    (:`then_1`
      (if (`StrixReplicatorComponent.GetIsOwner` (`self.StrixReplicator`))
        (bind _returnvalue (`|CreateWidget` "/Game/Scene/MainMenu/WB_MainMenu2.WB_MainMenu2_C" null self))
        (bind _output_get (set `self.UI` _returnvalue))
        (`UserWidget.AddToViewport` _output_get 0)))
    (:`then_2`
      (if (`StrixReplicatorComponent.GetIsOwner` (`self.StrixReplicator`))
        (bind _asgame_instance_main (cast `/Game/Scene/Game_Instance_Main` (`GameplayStatics.GetGameInstance`)))
        (`KismetArrayLibrary.Array_Clear` (`/Game/Scene/Game_Instance_Main.Player Infos` _asgame_instance_main))
        (set `self.playerName` (`/Game/Scene/Game_Instance_Main.name` _asgame_instance_main))
        (set `self.ID` (`/Game/Scene/Game_Instance_Main.ID` _asgame_instance_main))
        (`StrixBlueprintFunctionLibrary.SendRpcToRoomOwner` null "SetMember" (`|MakeArray` (`StrixBlueprintFunctionLibrary.Conv_IntToStrixRelayArg` (`self.ID`)) (`StrixBlueprintFunctionLibrary.Conv_StringToStrixRelayArg` (`self.playerName`))))))
    (:`then_3`
      (`KismetSystemLibrary.Delay` 5.0)
      (`self.SetMatrial`)
      (`self.SetName`))
    (:`then_4`
      (`self.point`))))

(event `SetMember`
  (params (ID :type Integer) (name :type String))
  (bind _returnvalue (`StrixBlueprintFunctionLibrary.GetCurrentRoomMemberById` 0 ID))
  (bind _asgame_instance_main (cast `/Game/Scene/Game_Instance_Main` (`GameplayStatics.GetGameInstance`)))
  (bind _id (break `StrixRoomMember` _returnvalue))
  (bind _room_id (`/Game/Scene/Game_Instance_Main.Connect` _asgame_instance_main _id))
  (set `self.RoomID` _room_id)
  (`/Game/Scene/Game_Instance_Main.Set Name` _asgame_instance_main _id (`KismetStringLibrary.Conv_StringToName` name))
  (for _array_element (`/Game/Scene/Game_Instance_Main.Player Infos` _asgame_instance_main)
    (`StrixBlueprintFunctionLibrary.SendRpcToOtherMembers` null "SetOtherMember" (`|MakeArray` (`StrixBlueprintFunctionLibrary.Conv_IntToStrixRelayArg` (break `/Game/DataTable/Struct/S_PlayerInfo` _array_element)) (`StrixBlueprintFunctionLibrary.Conv_StringToStrixRelayArg` (`KismetStringLibrary.Conv_NameToString` (`.Name_5_6B24B1704D3EDBC0825E2EA4B9B893DF` (break `/Game/DataTable/Struct/S_PlayerInfo` _array_element))))))))

(event `SetOtherMember`
  (params (ID :type Integer) (Name :type String))
  (bind _asgame_instance_main (cast `/Game/Scene/Game_Instance_Main` (`GameplayStatics.GetGameInstance`)))
  (`/Game/Scene/Game_Instance_Main.Connect` _asgame_instance_main ID)
  (`/Game/Scene/Game_Instance_Main.Set Name` _asgame_instance_main ID (`KismetStringLibrary.Conv_StringToName` Name)))

(event `COUNT`
  (bind _asgame_instance_main (cast `/Game/Scene/Game_Instance_Main` (`GameplayStatics.GetGameInstance`)))
  (if (`self.ready`)
    (`/Game/Scene/Game_Instance_Main.EraseCount` _asgame_instance_main)
    (set `self.ready` false)
    (else
      (`/Game/Scene/Game_Instance_Main.Add Count` _asgame_instance_main)
      (set `self.ready` true))))

(event `GoToLevel`
  (`GameplayStatics.OpenLevelBySoftObjectPtr` "/Game/Scene/Game/Map/PersistentLevel.PersistentLevel"))

(event `PushPlayButton`
  ;[1 1 1] 開始ボタンを押したときの処理
  (bind _returnvalue (`StrixBlueprintFunctionLibrary.IsRoomOwner` 0))
  (if _returnvalue
    (bind _allready (`self.CheckReady`))
    (if _allready
      (`StrixBlueprintFunctionLibrary.SendRpcToAll` null "GoToLevel")
      (else
        (`KismetSystemLibrary.PrintString` "まだ準備中のプレイヤーがいます")))
    (else
      (`KismetSystemLibrary.RetriggerableDelay` 0.1)
      (`StrixBlueprintFunctionLibrary.SendRpcToAll` null "COUNT")
      (`KismetSystemLibrary.Delay` 0.1)
      (if (`self.ready`)
        (`self.SetUIText_T`)
        (else
          (`self.SetUIText_F`))))))

(event `SetUIText_T`
  (bind _ui (`self.UI`)
    (:`then`
      (`TextBlock.SetText` (`/Game/Scene/MainMenu/WB_MainMenu2.PlayText` _ui) "Waiting for others..."))
    (:`else`)))

(event `SetUIText_F`
  (bind _ui (`self.UI`)
    (:`then`
      (`TextBlock.SetText` (`/Game/Scene/MainMenu/WB_MainMenu2.PlayText` _ui) "Ready?"))
    (:`else`)))

(event `Remove`
  (params (ID :type Integer))
  ;[1 1 1] ルームから抜ける処理
  (bind _asgame_instance_main (cast `/Game/Scene/Game_Instance_Main` (`GameplayStatics.GetGameInstance`)))
  (`/Game/Scene/Game_Instance_Main.Cutting` _asgame_instance_main ID)
  (`KismetSystemLibrary.Delay` 5.0)
  (`self.SetMatrial`)
  (if (`StrixReplicatorComponent.GetIsOwner` (`self.StrixReplicator`))
    (bind _roomid (`/Game/Scene/Game_Instance_Main.IDtoRoomIDConvert` _asgame_instance_main (`self.ID`)))
    (bind _outactors (`GameplayStatics.GetAllActorsWithTag` (`KismetStringLibrary.Conv_StringToName` (`KismetStringLibrary.Conv_IntToString` _roomid))))
    (if (>= (`KismetArrayLibrary.Array_Length` _outactors) 1)
      (`self.K2_SetActorLocation` (`self.K2_GetActorLocation` (`|GetArrayItem` _outactors))))))

(event `PushRemovebutton`
  ;[1 1 1] ルームから抜ける処理
  (bind _asgame_instance_main (cast `/Game/Scene/Game_Instance_Main` (`GameplayStatics.GetGameInstance`)))
  (`StrixBlueprintFunctionLibrary.SendRpcToAll` null "Remove" (`|MakeArray` (`StrixBlueprintFunctionLibrary.Conv_IntToStrixRelayArg` (`/Game/Scene/Game_Instance_Main.ID` _asgame_instance_main)))))

(event `self.ReceiveTick`
  (params (DeltaSeconds :type "Float (single-precision)"))
  (`self.SetMatrial`)
  (bind _returnvalue (`StrixBlueprintFunctionLibrary.IsRoomOwner` 0))
  (if (and _returnvalue (`StrixReplicatorComponent.GetIsOwner` (`self.StrixReplicator`)))
    (set `self.ready` true)))

(fn `CheckReady`
  (returns (AllReady :type Boolean))
  (bind _returnvalue (`StrixBlueprintFunctionLibrary.IsRoomOwner` 0))
  (if _returnvalue
    (bind _outactors (`GameplayStatics.GetAllActorsOfClass` "BP_LobbyCleric_C"))
    (for _array_element _outactors
      (if (not (`/Game/Scene/MainMenu/BP_LobbyCleric.ready` _array_element))
        (return false)))
    (return true)
    (else
      (return false))))

(fn `OnRep_playerName`
  (bind _aswbp_text (cast `/Game/UI/Cleric_UI/WBP_Text` (`WidgetComponent.GetWidget` (`self.Widget`))))
  (`/Game/UI/Cleric_UI/WBP_Text.SetText` _aswbp_text (`self.playerName`)))

(fn `Point`
  (if (not (`StrixReplicatorComponent.GetIsOwner` (`self.StrixReplicator`)))
    (for _index (range 1 4) :!label _label
      (bind _outactors (`GameplayStatics.GetAllActorsWithTag` (`KismetStringLibrary.Conv_StringToName` (`KismetStringLibrary.Conv_IntToString` _index))))
      (for _array_element _outactors
        (`KismetSystemLibrary.PrintString` (`KismetSystemLibrary.GetDisplayName` _array_element) true true (struct :`G` 0.66 :`B` 1.0 :`A` 1.0) 10.0)
        (bind _asplayer_state_lobby (cast `/Game/Scene/MainMenu/playerState_lobby` _array_element))
        (if (not (`/Game/Scene/MainMenu/playerState_lobby.IsPlayer` _asplayer_state_lobby))
          (`self.K2_SetActorTransform` (`self.GetTransform` _asplayer_state_lobby))
          (set `/Game/Scene/MainMenu/playerState_lobby.cleric` self _asplayer_state_lobby)
          (set `/Game/Scene/MainMenu/playerState_lobby.IsPlayer` true _asplayer_state_lobby)
          (goto _label :!via `Break`))))))

(fn `UserConstructionScript`)