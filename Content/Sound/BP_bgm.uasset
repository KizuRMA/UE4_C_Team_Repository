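; BP_bgm is a background music actor that plays a configurable Sound on its Audio component.
; It sets the sound on BeginPlay and exposes FadeIn, FadeOut and AdjustVolume events that take a fade time.
; Target volume is master volume times BGM volume, read from Game_Instance_Main through a cast helper.
; AdjustVolume also starts playback with an instant fade-in if the audio is not playing.
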(event `self.ReceiveBeginPlay`
  (`AudioComponent.SetSound` (`self.Audio`) (`self.sound`)))

(event `FadeIn`
  (params (time :type "Float (double-precision)"))
  (bind _gameinstance_main (`self.GetGameInstance`)
    (:`then`
      (`AudioComponent.FadeIn` (`self.Audio`) time (* (`/Game/Scene/Game_Instance_Main.MasterVolume` _gameinstance_main) (`/Game/Scene/Game_Instance_Main.BGMVolume` _gameinstance_main)) 0.0 "Linear"))))

(event `FadeOut`
  (params (time :type "Float (double-precision)"))
  (`AudioComponent.FadeOut` (`self.Audio`) time 0.0 "Linear"))

(event `AdjustVolume`
  (params (time :type "Float (double-precision)"))
  (bind _gameinstance_main (`self.GetGameInstance`)
    (:`then`
      (`AudioComponent.AdjustVolume` (`self.Audio`) time (* (`/Game/Scene/Game_Instance_Main.MasterVolume` _gameinstance_main) (`/Game/Scene/Game_Instance_Main.BGMVolume` _gameinstance_main)) "Linear")
      (if (not (`AudioComponent.IsPlaying` (`self.Audio`)))
        (`self.FadeIn` 0.0)))))

(fn `UserConstructionScript`)