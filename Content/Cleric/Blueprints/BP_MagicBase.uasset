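; BP_MagicBase is the Cleric's magic spell actor, a projectile that damages what it hits and expires five seconds after spawning.
; Damage and damage type come from DT_MagicSpellTable by SpellName: blocking hits damage and destroy it, while overlaps damage without destroying it.
; SpawnPoint places it at the target or staff per MagicSpawnType, then realigns projectile velocity to its forward vector.
; An overlapping-enemy damage loop is present but unconnected.
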(event `self.ReceiveBeginPlay`
  (`KismetSystemLibrary.Delay` 5.0)
  (`self.K2_DestroyActor`))

(event `self.ReceiveHit`
  (params (MyComp :type "PrimitiveComponent Object Reference") (Other :type "Actor Object Reference") (OtherComp :type "PrimitiveComponent Object Reference") (bSelfMoved :type Boolean) (HitLocation :type "Vector Structure") (HitNormal :type "Vector Structure") (NormalImpulse :type "Vector Structure") (Hit :type "HitResult Structure (by ref)"))
  ;[1 1 1] コリジョンタイプがブロック時
  (bind _returnvalue (`|GetDataTableRow` "/Game/Cleric/UI/DataTables/DT_MagicSpellTable.DT_MagicSpellTable" (`self.Spell Name`))
    (:`then`
      (bind (_particle _damage _damagetype) (break `/Game/Cleric/UI/Struct/S_MagicSpell` _returnvalue))
      (`GameplayStatics.ApplyDamage` Other _damage (`self.GetInstigatorController`) null _damagetype)
      (`self.K2_DestroyActor`))))

(event `self.ReceiveActorBeginOverlap`
  (params (OtherActor :type "Actor Object Reference"))
  ;[1 1 1] コリジョンタイプがオーバーラップ時
  (bind _returnvalue (`|GetDataTableRow` "/Game/Cleric/UI/DataTables/DT_MagicSpellTable.DT_MagicSpellTable" (`self.Spell Name`))
    (:`then`
      (bind (_particle _damage _damagetype) (break `/Game/Cleric/UI/Struct/S_MagicSpell` _returnvalue))
      (`GameplayStatics.ApplyDamage` OtherActor _damage (`self.GetInstigatorController`) null _damagetype))))

(event `self.ReceiveTick`
  (params (DeltaSeconds :type "Float (single-precision)")))

(fn `Spawn Point`
  (params (TargetPos :type "Vector Structure") (StaffPos :type "Vector Structure") (Rotation :type "Rotator Structure"))
  (bind _projectilemovement (`self.ProjectileMovement`))
  (switch `/Game/Cleric/Blueprints/EBP_MagicSpawnType` (`self.MagicSpawnType`)
    (:`NewEnumerator3`
      (`self.K2_SetActorTransform` self (`KismetMathLibrary.MakeTransform` TargetPos) false false))
    (:`NewEnumerator4`
      (`self.K2_SetActorTransform` self (`KismetMathLibrary.MakeTransform` StaffPos Rotation) false false)))
  ;[1 1 1] Projectailを新しいTransformに合わせる
  (set `MovementComponent.Velocity` (* (`self.GetActorForwardVector` self) (`ProjectileMovementComponent.InitialSpeed` _projectilemovement)) _projectilemovement))

(fn `UserConstructionScript`)