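; Base Blueprint for a magic stone, holding its magic attribute in a BP_MagicInfo object and showing the matching mesh.
; On BeginPlay it creates that object and fills its definition from the DT_MagicDefineTable row named by MagicTypeName.
; SetMagicInfoAndVisual swaps in another info object and sets the Sphere mesh from its table row.
; Tick polls for a type name mismatch, then updates the mesh and MagicTypeName to follow the info.
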(event `self.ReceiveBeginPlay`
  ;[1 1 1] 魔石の情報クラスに属性を入れる
  (bind _returnvalue (`|GenericCreateObject` "/Game/Cleric/UI/MagicSlot/BP_MagicInfo.BP_MagicInfo_C" self))
  (bind _returnvalue_2 (`|GetDataTableRow` "/Game/Cleric/UI/DataTables/DT_MagicDefineTable.DT_MagicDefineTable" (`self.Magic Type Name`))
    (:`then`
      (set `/Game/Cleric/UI/MagicSlot/BP_MagicInfo.Magic Info Difine` (`.MagicInfoDifine_36_69F1A7CE4DA11F35F152749B8340C8A0` (break `/Game/Cleric/UI/Struct/S_MagicDifine` _returnvalue_2)) _returnvalue)
      (set `self.Magic Info` _returnvalue))))

(event `Set Magic Info And Visual`
  (params (`Magic Info` :type "/Game/Cleric/UI/MagicSlot/BP_MagicInfo Object Reference"))
  (bind _output_get (set `self.Magic Info` `Magic Info`))
  (bind _magic_info_difine_name (break `/Game/Cleric/UI/Struct/S_MagicInfoDifine` (`/Game/Cleric/UI/MagicSlot/BP_MagicInfo.Magic Info Difine` _output_get)))
  (bind _returnvalue (`|GetDataTableRow` "/Game/Cleric/UI/DataTables/DT_MagicDefineTable.DT_MagicDefineTable" _magic_info_difine_name)
    (:`then`
      (`StaticMeshComponent.SetStaticMesh` (`self.Sphere`) (`.MagicStoneMesh_40_E89B644F4516B67A7481D2A2FF4C27B8` (break `/Game/Cleric/UI/Struct/S_MagicDifine` _returnvalue))))))

(event `self.ReceiveTick`
  (params (DeltaSeconds :type "Float (single-precision)"))
  (bind _magic_info_difine_name (break `/Game/Cleric/UI/Struct/S_MagicInfoDifine` (`/Game/Cleric/UI/MagicSlot/BP_MagicInfo.Magic Info Difine` (`self.Magic Info`))))
  (bind _magic_info_difine_name_2 (break `/Game/Cleric/UI/Struct/S_MagicInfoDifine` (`/Game/Cleric/UI/MagicSlot/BP_MagicInfo.Magic Info Difine` (`self.Magic Info`))))
  (if (!= (`self.Magic Type Name`) _magic_info_difine_name_2)
    (bind _returnvalue (`|GetDataTableRow` "/Game/Cleric/UI/DataTables/DT_MagicDefineTable.DT_MagicDefineTable" _magic_info_difine_name)
      (:`then`
        (`StaticMeshComponent.SetStaticMesh` (`self.Sphere`) (`.MagicStoneMesh_40_E89B644F4516B67A7481D2A2FF4C27B8` (break `/Game/Cleric/UI/Struct/S_MagicDifine` _returnvalue)))
        (set `self.Magic Type Name` _magic_info_difine_name)))))

(fn `UserConstructionScript`)