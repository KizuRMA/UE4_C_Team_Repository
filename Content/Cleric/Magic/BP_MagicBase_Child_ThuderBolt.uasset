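; Cleric thunderbolt spell actor, a child in the MagicBase family, that triggers a delayed lightning hit where it stands.
; On BeginPlay it waits briefly, spawns a separate ThunderBoltHit actor at its own transform, and in parallel runs a longer timer before destroying itself.
; Hit and overlap events only forward to the parent class.
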(event `self.ReceiveBeginPlay`
  (`|ExecutionSequence`
    (:`then_0`
      (`KismetSystemLibrary.Delay` 0.2)
      (`|SpawnActorFromClass` "/Game/Cleric/Magic/BP_MagicBase_Child_ThunderBoltHit.BP_MagicBase_Child_ThunderBoltHit_C" (`self.GetTransform`) "Undefined" "OverrideRootScale" null null))
    (:`then_1`
      (`KismetSystemLibrary.Delay` 4.0)
      (`self.K2_DestroyActor`))))

(event `self.ReceiveHit`
  (params (MyComp :type "PrimitiveComponent Object Reference") (Other :type "Actor Object Reference") (OtherComp :type "PrimitiveComponent Object Reference") (bSelfMoved :type Boolean) (HitLocation :type "Vector Structure") (HitNormal :type "Vector Structure") (NormalImpulse :type "Vector Structure") (Hit :type "HitResult Structure (by ref)"))
  (`parent.ReceiveHit` MyComp Other OtherComp bSelfMoved HitLocation HitNormal NormalImpulse Hit))

(event `self.ReceiveActorBeginOverlap`
  (params (OtherActor :type "Actor Object Reference"))
  (`parent.ReceiveActorBeginOverlap` OtherActor))

(fn `UserConstructionScript`
  (`parent.UserConstructionScript`))