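; Base magic spell actor that deals damage and type from DT_MagicSpellTable by SpellName.
; Blocking hits damage and destroy it; overlaps damage immediately, then Tick damages overlapping actors every frame unless held in EnemyArray's 0.5-second grace list.
; SpawnPoint places it at target or staff by MagicSpawnType and realigns projectile velocity.
; It expires after five seconds or particle completion, and a Strix RPC toggles particle ticking on sync.
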(event `self.ReceiveBeginPlay`
  (`KismetSystemLibrary.Delay` 5.0)
  (`self.K2_DestroyActor`))

(event `self.ReceiveHit`
  (params (MyComp :type "PrimitiveComponent Object Reference") (Other :type "Actor Object Reference") (OtherComp :type "PrimitiveComponent Object Reference") (bSelfMoved :type Boolean) (HitLocation :type "Vector Structure") (HitNormal :type "Vector Structure") (NormalImpulse :type "Vector Structure") (Hit :type "HitResult Structure (by ref)"))
  ;[1 1 1] コリジョンタイプがブロック時
  (bind _returnvalue (`|GetDataTableRow` "/Game/Cleric/UI/DataTables/DT_MagicSpellTable.DT_MagicSpellTable" (`self.Spell Name`))
    (:`then`
      (bind (_particle _damage _damagetype) (break `/Game/Cleric/UI/Struct/S_MagicSpell` _returnvalue))
      (`GameplayStatics.ApplyDamage` Other _damage (`self.GetInstigatorController`) null _damagetype)
      (`self.K2_DestroyActor`))))

(event `self.ReceiveActorBeginOverlap`
  (params (OtherActor :type "Actor Object Reference"))
  ;[1 1 1] コリジョンタイプがオーバーラップ時
  (bind _returnvalue (`|GetDataTableRow` "/Game/Cleric/UI/DataTables/DT_MagicSpellTable.DT_MagicSpellTable" (`self.Spell Name`))
    (:`then`
      (bind (_particle _damage _damagetype) (break `/Game/Cleric/UI/Struct/S_MagicSpell` _returnvalue))
      (`GameplayStatics.ApplyDamage` OtherActor _damage (`self.GetInstigatorController`) null _damagetype)
      (`KismetArrayLibrary.Array_AddUnique` (`self.Enemy Array`) OtherActor)
      (`KismetSystemLibrary.Delay` 0.5)
      (`KismetArrayLibrary.Array_RemoveItem` (`self.Enemy Array`) OtherActor))))

(event `self.ReceiveTick`
  (params (DeltaSeconds :type "Float (single-precision)"))
  ;[1 1 1] overlap し続けている敵に継続ダメージ
  (for _array_element (`PrimitiveComponent.GetOverlappingActors` (`self.CollisionSphere`) null)
    (if (== (`KismetArrayLibrary.Array_Find` (`self.Enemy Array`) _array_element) -1)
      (bind _returnvalue (`|GetDataTableRow` "/Game/Cleric/UI/DataTables/DT_MagicSpellTable.DT_MagicSpellTable" (`self.Spell Name`))
        (:`then`
          (bind (_particle _damage _damagetype) (break `/Game/Cleric/UI/Struct/S_MagicSpell` _returnvalue))
          (`GameplayStatics.ApplyDamage` _array_element _damage (`self.GetInstigatorController`) null _damagetype))))))

(event `self.ParticleSystem.OnSystemFinished`
  (params (PSystem :type "ParticleSystemComponent Object Reference"))
  ;[1 1 1] 魔法が終了したら削除する
  (`self.K2_DestroyActor`))

(event `self.StrixReplicator.OnSyncBegin`
  (`StrixBlueprintFunctionLibrary.RegisterStrixRpc` null "Playereffect")
  (`StrixBlueprintFunctionLibrary.SendRpcToAll` null "Playereffect"))

(event `Playereffect`
  (bind _particlesystem (`self.ParticleSystem`))
  (`ActorComponent.SetComponentTickEnabled` _particlesystem false)
  (`ActorComponent.SetComponentTickEnabled` _particlesystem true)
  (`KismetSystemLibrary.PrintString` "Hello"))

(fn `Spawn Point`
  (params (TargetPos :type "Vector Structure") (StaffPos :type "Vector Structure") (Rotation :type "Rotator Structure"))
  (bind _projectilemovement (`self.ProjectileMovement`))
  (switch `/Game/Cleric/Blueprints/EBP_MagicSpawnType` (`self.MagicSpawnType`)
    (:`NewEnumerator3`
      (`self.K2_SetActorTransform` self (`KismetMathLibrary.MakeTransform` TargetPos) false false))
    (:`NewEnumerator4`
      (`self.K2_SetActorTransform` self (`KismetMathLibrary.MakeTransform` StaffPos Rotation) false false)))
  ;[1 1 1] Projectailを新しいTransformに合わせる
  (set `MovementComponent.Velocity` (* (`self.GetActorForwardVector` self) (`ProjectileMovementComponent.InitialSpeed` _projectilemovement)) _projectilemovement))

(fn `UserConstructionScript`)