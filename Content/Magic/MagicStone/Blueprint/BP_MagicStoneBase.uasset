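; Base magic stone actor that launches upward with random horizontal velocity when spawned and represents one magic type.
; BeginPlay builds a BP_MagicInfo object, using DT_MagicDefineTable for its mesh and any preset type's definition.
; Tick refreshes mesh and material when the type changes, and counts down lifetime while no BP_Cleric_new overlaps.
; An "Empty" type change or expired lifetime triggers a timeline-driven material "Rate" animation, then destroys the actor.
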(event `self.ReceiveTick`
  (params (DeltaSeconds :type "Float (single-precision)"))
  (bind _sphere (`self.Sphere`))
  (bind _magic_info_difine_name (break `/Game/DataTable/Struct/S_MagicInfoDifine` (`/Game/UI/Cleric_UI/MagicSlot/BP_MagicInfo.Magic Info Difine` (`self.Magic Info`))))
  (bind _magic_info_difine_name_2 (break `/Game/DataTable/Struct/S_MagicInfoDifine` (`/Game/UI/Cleric_UI/MagicSlot/BP_MagicInfo.Magic Info Difine` (`self.Magic Info`))))
  ;[1 1 1] 更新処理
  (`|ExecutionSequence`
    (:`then_0`
      (if (!= (`self.Magic Type Name`) _magic_info_difine_name_2)
        (bind _returnvalue (`|GetDataTableRow` "/Game/DataTable/DT_MagicDefineTable.DT_MagicDefineTable" _magic_info_difine_name)
          (:`then`
            (bind (_combomagicspell _combomagicspawninfo _strongmagicspell _strongmagicspawninfo _magicinfodifine _magicstonemesh) (break `/Game/DataTable/Struct/S_MagicDifine` _returnvalue))
            (`StaticMeshComponent.SetStaticMesh` _sphere _magicstonemesh)
            (`PrimitiveComponent.SetMaterial` _sphere 0 (`StaticMesh.GetMaterial` _magicstonemesh 0))
            (bind _returnvalue_2 (`PrimitiveComponent.CreateDynamicMaterialInstance` (`self.Sphere`) 0 null "None"))
            (set `self.Material` _returnvalue_2)
            (bind _output_get (set `self.Magic Type Name` _magic_info_difine_name_2))
            (if (== _output_get "Empty")
              (`self.Destory Anim`))))))
    (:`then_1`
      (if (not (>= (`KismetArrayLibrary.Array_Length` (`PrimitiveComponent.GetOverlappingActors` (`self.Sphere2`) "/Game/Character/Cleric/BP_Cleric_new.BP_Cleric_new_C")) 1))
        (bind _output_get_2 (set `self.LifeTime` (- (`self.LifeTime`) (`GameplayStatics.GetWorldDeltaSeconds`))))
        (if (<= _output_get_2 0.0)
          (`self.Destory Anim`))))))

(event `self.ReceiveBeginPlay`
  ;[1 1 1] 初期化処理
  (`self.Setup Magic Info`)
  (`self.Projectile Random Velocity`)
  (bind _returnvalue (`PrimitiveComponent.CreateDynamicMaterialInstance` (`self.Sphere`) 0 null "None"))
  (set `self.Material` _returnvalue))

(event `Projectile Random Velocity`
  ;[1 1 1] プロジェクタイルの移動方向をランダム化
  (`ProjectileMovementComponent.SetVelocityInLocalSpace` (`self.ProjectileMovement`) (`KismetMathLibrary.MakeVector` (* (`KismetMathLibrary.RandomFloatInRange` -1.0 1.0) 250.0) (* (`KismetMathLibrary.RandomFloatInRange` -1.0 1.0) 250.0) 500.0)))

(event `Destory Anim`
  (bind (_direction `_新規track_0`) (`Timeline|タイムライン_0`)
    (:`Update`
      (`MaterialInstanceDynamic.SetScalarParameterValue` (`self.Material`) "Rate" `_新規track_0`))
    (:`Finished`
      (`self.K2_DestroyActor`))))

(fn `Setup Magic Info`
  (bind _magic_type_name (`self.Magic Type Name`))
  (if (not (== _magic_type_name "Empty"))
    (bind _returnvalue (`|GetDataTableRow` "/Game/DataTable/DT_MagicDefineTable.DT_MagicDefineTable" _magic_type_name)
      (:`then`
        (bind (_name _icon _increaseability) (break `/Game/DataTable/Struct/S_MagicInfoDifine` (`.MagicInfoDifine_36_69F1A7CE4DA11F35F152749B8340C8A0` (break `/Game/DataTable/Struct/S_MagicDifine` _returnvalue))))
        (set `self.Magic Info Difine` (make `/Game/DataTable/Struct/S_MagicInfoDifine` _name _icon _increaseability 2)))))
  (bind _returnvalue_2 (`|GenericCreateObject` "/Game/UI/Cleric_UI/MagicSlot/BP_MagicInfo.BP_MagicInfo_C" self (`self.Magic Info Difine`)))
  (bind _magic_info_difine_name (break `/Game/DataTable/Struct/S_MagicInfoDifine` (`/Game/UI/Cleric_UI/MagicSlot/BP_MagicInfo.Magic Info Difine` _returnvalue_2)))
  (bind _returnvalue_3 (`|GetDataTableRow` "/Game/DataTable/DT_MagicDefineTable.DT_MagicDefineTable" _magic_info_difine_name)
    (:`then`
      (set `self.Magic Info` _returnvalue_2)
      (`StaticMeshComponent.SetStaticMesh` (`self.Sphere`) (`.MagicStoneMesh_40_E89B644F4516B67A7481D2A2FF4C27B8` (break `/Game/DataTable/Struct/S_MagicDifine` _returnvalue_3)))
      (set `self.Magic Type Name` _magic_info_difine_name)
      (return))))

(fn `UserConstructionScript`)