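; Base enemy breath spell projectile that damages ThirdPersonCharacter_sato targets using its DT_MagicSpellTable damage value.
; Owner-detected overlaps RPC HitFunctiom, which sends Damage to the hit member, triggers hit effects, deletes one-hit spells and holds the target in EnemyArray briefly.
; Outside a Strix room, Tick directly damages overlapping characters absent from that array.
; SpawnPoint places and scales the actor, realigning projectile velocity to its forward vector.
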(event `self.HitFunctiom`
  ;[1 1 1] ダメージを与える処理
  (bind _returnvalue (`|GetDataTableRow` "/Game/DataTable/DT_MagicSpellTable.DT_MagicSpellTable" (`self.Spell Name`))
    (:`then`
      (bind _asthird_person_character_sato (cast `/Game/Scene/TestMaps/l/ThirdPersonCharacter_sato` (`self.HitActor`)))
      (bind _returnvalue_2 (`StrixBlueprintFunctionLibrary.GetCurrentRoomMemberById` 0 (`/Game/Scene/TestMaps/l/ThirdPersonCharacter_sato.MemberID` _asthird_person_character_sato)))
      (`StrixBlueprintFunctionLibrary.SendRpc` _asthird_person_character_sato _returnvalue_2 "Damage" (`|MakeArray` (`StrixBlueprintFunctionLibrary.Conv_FloatToStrixRelayArg` (`.Damage_5_27260A5F4195EB1407AA7886E6EF968A` (break `/Game/DataTable/Struct/S_MagicSpell` _returnvalue)))))
      (`KismetArrayLibrary.Array_AddUnique` (`self.Enemy Array`) (`self.HitActor`))
      (`|ExecutionSequence`
        (:`then_0`
          ;[1 1 1] ヒット時のネット・ローカル処理
          (bind _returnvalue_3 (`StrixBlueprintFunctionLibrary.IsRoomServerConnected` 0))
          (if _returnvalue_3
            (`StrixBlueprintFunctionLibrary.SendRpcToAll` null "HitEffect")
            (if (`self.IsOneHit`)
              (`StrixBlueprintFunctionLibrary.SendRpcToAll` null "delete"))
            (else
              (`self.HitEffect`)
              (if (`self.IsOneHit`)
                (`self.delete`)))))
        (:`then_1`
          (`KismetSystemLibrary.Delay` 0.5)
          (`KismetArrayLibrary.Array_RemoveItem` (`self.Enemy Array`) (`self.HitActor`)))))))

(event `self.ReceiveActorBeginOverlap`
  (params (OtherActor :type "Actor Object Reference"))
  ;[1 1 1] 敵と衝突時　ネット・ローカル処理
  (if (`StrixReplicatorComponent.GetIsOwner` (`self.StrixReplicator`))
    (set `self.HitActor` OtherActor)
    (`StrixBlueprintFunctionLibrary.SendRpcToObjectOwner` null "HitFunctiom")))

(event `self.ReceiveTick`
  (params (DeltaSeconds :type "Float (single-precision)"))
  ;[1 1 1] overlap し続けている敵に継続ダメージ
  (bind _returnvalue (`StrixBlueprintFunctionLibrary.IsRoomServerConnected` 0))
  (if (not _returnvalue)
    (bind _returnvalue_2 (`|GetDataTableRow` "/Game/DataTable/DT_MagicSpellTable.DT_MagicSpellTable" (`self.Spell Name`))
      (:`then`
        (for _array_element (`PrimitiveComponent.GetOverlappingActors` (`self.CollisionSphere`) null)
          (if (== (`KismetArrayLibrary.Array_Find` (`self.Enemy Array`) _array_element) -1)
            (bind _asthird_person_character_sato (cast `/Game/Scene/TestMaps/l/ThirdPersonCharacter_sato` _array_element))
            (`/Game/Scene/TestMaps/l/ThirdPersonCharacter_sato.Damage` _asthird_person_character_sato (`.Damage_5_27260A5F4195EB1407AA7886E6EF968A` (break `/Game/DataTable/Struct/S_MagicSpell` _returnvalue_2)))))))))

(fn `Spawn Point`
  (params (TargetPos :type "Vector Structure") (StaffPos :type "Vector Structure") (Rotation :type "Rotator Structure"))
  (bind _projectilemovement (`self.ProjectileMovement`))
  (`self.K2_SetActorTransform` self (`KismetMathLibrary.MakeTransform` StaffPos Rotation (2.0 2.0 2.0)) false false)
  ;[1 1 1] Projectailを新しいTransformに合わせる
  (set `MovementComponent.Velocity` (* (`self.GetActorForwardVector` self) (`ProjectileMovementComponent.InitialSpeed` _projectilemovement)) _projectilemovement))

(fn `UserConstructionScript`
  (`parent.UserConstructionScript`))