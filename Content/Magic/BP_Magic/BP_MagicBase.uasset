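; Base magic spell actor that damages BP_Enemy on overlap, taking damage and effect classes from DT_MagicSpellTable by SpellName.
; EnemyArray briefly blocks repeat hits, one-hit spells destroy themselves, and all expire after Duration.
; When connected, Strix RPCs route hits to the owner and broadcast effects and deletion; offline these run locally, with Tick damaging overlapping enemies.
; SpawnPoint either grounds the spell at the target or launches it from the staff.
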(event `HitFunctiom`
  ;[1 1 1] ダメージを与える処理
  (if (== (`KismetArrayLibrary.Array_Find` (`self.Enemy Array`) (`self.HitActor`)) -1)
    (bind _returnvalue (`|GetDataTableRow` "/Game/DataTable/DT_MagicSpellTable.DT_MagicSpellTable" (`self.Spell Name`))
      (:`then`
        (bind _asbp_enemy (cast `/Enemy/Enemy/BP/BP_Enemy` (`self.HitActor`))
          (:`then`
            (`/Engine/EditorBlueprintResources/StandardMacros.IsValid` _asbp_enemy
              (:`Is Valid`
                (`/Enemy/Enemy/BP/BP_Enemy.Damage` _asbp_enemy (`.Damage_5_27260A5F4195EB1407AA7886E6EF968A` (break `/Game/DataTable/Struct/S_MagicSpell` _returnvalue)) (`self.memberID`) (`KismetMathLibrary.MakeVector` 1.0)))
              (:`Is Not Valid`
                _)))
          (:`CastFailed`
            _))
        (`KismetArrayLibrary.Array_AddUnique` (`self.Enemy Array`) (`self.HitActor`))
        ;[1 1 1] ヒット時のネット・ローカル処理
        (`|ExecutionSequence`
          (:`then_0`
            (bind _returnvalue_2 (`StrixBlueprintFunctionLibrary.IsRoomServerConnected` 0))
            (if _returnvalue_2
              (`StrixBlueprintFunctionLibrary.SendRpcToAll` null "HitEffect")
              (if (`self.IsOneHit`)
                (`StrixBlueprintFunctionLibrary.SendRpcToAll` null "delete"))
              (else
                (`self.HitEffect`)
                (if (`self.IsOneHit`)
                  (`self.delete`)))))
          (:`then_1`
            (`KismetSystemLibrary.Delay` 0.5)
            (`KismetArrayLibrary.Array_RemoveItem` (`self.Enemy Array`) (`self.HitActor`))))))))

(event `self.ReceiveActorEndOverlap`
  (params (OtherActor :type "Actor Object Reference"))
  (`KismetArrayLibrary.Array_RemoveItem` (`self.Enemy Array`) OtherActor))

(event `self.ReceiveActorBeginOverlap`
  (params (OtherActor :type "Actor Object Reference"))
  ;[1 1 1] 敵と衝突時　ネット・ローカル処理
  (bind _returnvalue (`StrixBlueprintFunctionLibrary.IsRoomServerConnected` 0))
  (if _returnvalue
    (set `self.HitActor` OtherActor)
    (`StrixBlueprintFunctionLibrary.SendRpcToObjectOwner` null "HitFunctiom")
    (else
      (set `self.HitActor` OtherActor)
      (`self.HitFunctiom`))))

(event `delete`
  (`self.K2_DestroyActor`))

(event `self.StrixReplicator.OnSyncBegin`
  (`|ExecutionSequence`
    (:`then_0`
      ;[1 1 1] 呼び出し関数の設定
      (`StrixBlueprintFunctionLibrary.RegisterStrixRpc` null "HitFunctiom")
      (`StrixBlueprintFunctionLibrary.RegisterStrixRpc` null "delete")
      (`StrixBlueprintFunctionLibrary.RegisterStrixRpc` null "HitEffect")
      (`StrixBlueprintFunctionLibrary.RegisterStrixRpc` null "MainEffect"))
    (:`then_1`
      ;[1 1 1] 一定時間経過したら削除
      (`KismetSystemLibrary.Delay` (`self.Duration`))
      (`KismetSystemLibrary.PrintString` "強制削除")
      (`StrixBlueprintFunctionLibrary.SendRpcToAll` null "delete"))
    (:`then_2`
      (if (`StrixReplicatorComponent.GetIsOwner` (`self.StrixReplicator`))
        (bind _returnvalue (`StrixBlueprintFunctionLibrary.IsRoomServerConnected` 0))
        (if _returnvalue
          (`StrixBlueprintFunctionLibrary.SendRpcToAll` null "MainEffect")
          (else
            (`self.MainEffect`)))))))

(event `MainEffect`
  ;[1 1 1] 魔法エフェクトを作成
  (bind _returnvalue (`|GetDataTableRow` "/Game/DataTable/DT_MagicSpellTable.DT_MagicSpellTable" (`self.Spell Name`))
    (:`then`
      (bind (_magic _damage _damagetype _baseeffect) (break `/Game/DataTable/Struct/S_MagicSpell` _returnvalue))
      (if (!= _baseeffect "/Game/Magic/BP_Effect/BP_Effectparent.BP_EffectParent_C")
        (bind _returnvalue_2 (`|SpawnActorFromClass` _baseeffect (`self.dummy`) "AdjustIfPossibleButAlwaysSpawn" "OverrideRootScale" null self null))
        (bind _output_get (set `self.BP_BaseEffect` _returnvalue_2))
        (`self.K2_AttachToActor` _output_get self "None" "SnapToTarget" "SnapToTarget" "KeepRelative" false)))))

(event `HitEffect`
  ;[1 1 1] 当たった時のエフェクトを作成
  (bind _returnvalue (`|GetDataTableRow` "/Game/DataTable/DT_MagicSpellTable.DT_MagicSpellTable" (`self.Spell Name`))
    (:`then`
      (bind (_magic _damage _damagetype _baseeffect _hiteffect) (break `/Game/DataTable/Struct/S_MagicSpell` _returnvalue))
      (if (!= _hiteffect "/Game/Magic/BP_Effect/BP_Effectparent.BP_EffectParent_C")
        (`|SpawnActorFromClass` _hiteffect (`self.GetTransform`) "Undefined" "OverrideRootScale" null null null)))))

(event `self.ReceiveBeginPlay`
  (bind _returnvalue (`StrixBlueprintFunctionLibrary.IsRoomServerConnected` 0))
  (if (not _returnvalue)
    (`self.MainEffect`)
    (`KismetSystemLibrary.Delay` (`self.Duration`))
    (`self.delete`)))

(event `self.ReceiveEndPlay`
  (params (EndPlayReason :type "EEndPlayReason Enum" :default "Destroyed"))
  (bind _bp_baseeffect (`self.BP_BaseEffect`)
    (:`then`
      (`/Game/Magic/BP_Effect/BP_Effectparent.Delete` _bp_baseeffect))
    (:`else`)))

(event `self.ReceiveTick`
  (params (DeltaSeconds :type "Float (single-precision)"))
  ;[1 1 1] overlap し続けている敵に継続ダメージ
  (bind _returnvalue (`StrixBlueprintFunctionLibrary.IsRoomServerConnected` 0))
  (if (not _returnvalue)
    (bind _returnvalue_2 (`|GetDataTableRow` "/Game/DataTable/DT_MagicSpellTable.DT_MagicSpellTable" (`self.Spell Name`))
      (:`then`
        (for _array_element (`PrimitiveComponent.GetOverlappingActors` (`self.CollisionSphere`) null)
          (if (== (`KismetArrayLibrary.Array_Find` (`self.Enemy Array`) _array_element) -1)
            (bind _asbp_enemy (cast `/Enemy/Enemy/BP/BP_Enemy` _array_element))
            (`/Enemy/Enemy/BP/BP_Enemy.Damage` _asbp_enemy (`.Damage_5_27260A5F4195EB1407AA7886E6EF968A` (break `/Game/DataTable/Struct/S_MagicSpell` _returnvalue_2)) (`self.memberID`) (`KismetMathLibrary.MakeVector` 1.0))))))))

(fn `Spawn Point`
  (params (TargetPos :type "Vector Structure") (StaffPos :type "Vector Structure") (Rotation :type "Rotator Structure"))
  (bind _projectilemovement (`self.ProjectileMovement`))
  (switch `/Game/DataTable/Enum/EBP_MagicSpawnType` (`self.MagicSpawnType`)
    (:`NewEnumerator3`
      (`self.K2_SetActorTransform` self (`KismetMathLibrary.MakeTransform` TargetPos) false false)
      (bind _outhit (`KismetSystemLibrary.LineTraceSingle` TargetPos (- TargetPos (0.0 0.0 5000.0)) "TraceTypeQuery3"))
      (bind (_bblockinghit _binitialoverlap _time _distance _location) (`GameplayStatics.BreakHitResult` _outhit))
      (if _bblockinghit
        (`self.K2_SetActorLocation` _location)))
    (:`NewEnumerator4`
      (`self.K2_SetActorTransform` self (`KismetMathLibrary.MakeTransform` StaffPos Rotation) false false :!label _label)
      ;[1 1 1] Projectailを新しいTransformに合わせる
      (set `MovementComponent.Velocity` (* (`self.GetActorForwardVector` self) (`ProjectileMovementComponent.InitialSpeed` _projectilemovement)) _projectilemovement))
    (:`NewEnumerator6`
      (goto _label))))

(fn `UserConstructionScript`)