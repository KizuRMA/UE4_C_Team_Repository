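; BP_MagicBase_Child_WindStorm is a wind storm spell child of the magic base that keeps itself placed on the surface below a stored point.
; Shortly after BeginPlay it saves its location as TargetLocation and prints it for debugging.
; Each tick it traces straight down from TargetLocation and teleportlessly moves the actor to any blocking hit, without sweeping.
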(event `self.ReceiveBeginPlay`
  (bind _returnvalue (`self.K2_GetActorLocation`))
  (`parent.ReceiveBeginPlay`)
  (`KismetSystemLibrary.Delay` 0.2)
  (set `self.TargetLocation` _returnvalue)
  (`KismetSystemLibrary.PrintString` (`KismetStringLibrary.Conv_VectorToString` _returnvalue)))

(event `self.ReceiveTick`
  (params (DeltaSeconds :type "Float (single-precision)"))
  (bind _targetlocation (`self.TargetLocation`))
  (`parent.ReceiveTick` DeltaSeconds)
  (bind _outhit (`KismetSystemLibrary.LineTraceSingle` _targetlocation (- _targetlocation (0.0 0.0 5000.0)) "TraceTypeQuery3"))
  (bind (_bblockinghit _binitialoverlap _time _distance _location) (`GameplayStatics.BreakHitResult` _outhit))
  (if _bblockinghit
    (`self.K2_SetActorLocation` _location)))

(fn `UserConstructionScript`
  (`parent.UserConstructionScript`))