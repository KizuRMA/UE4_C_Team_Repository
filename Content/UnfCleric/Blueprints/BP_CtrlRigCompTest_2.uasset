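; Test Blueprint that drives a skeletal mesh through a Control Rig component.
; The construction script maps the complete skeletal mesh to the rig.
; On the rig's pre-setup event, it loops over all socket names, which include bones, and copies each component-space location and rotation into the rig's initial bone transforms.
; BeginPlay, overlap and Tick events are empty.
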(event `self.ControlRig.OnPreSetupDelegate`
  (params (Component :type "ControlRigComponent Object Reference"))
  (for _array_element (`SceneComponent.GetAllSocketNames` (`self.SkeletalMesh`))
    (bind (_returnvalue_location _returnvalue_rotation) (`KismetMathLibrary.BreakTransform` (`SceneComponent.GetSocketTransform` (`self.SkeletalMesh`) _array_element "RTS_Component")))
    (`ControlRigComponent.SetInitialBoneTransform` (`self.ControlRig`) _array_element (`KismetMathLibrary.MakeTransform` _returnvalue_location _returnvalue_rotation) "ComponentSpace" false)))

(fn `UserConstructionScript`
  (locals (NewLocalVar_0 :type "Array of ControlRigComponentMappedBone Structure"))
  (`ControlRigComponent.AddMappedCompleteSkeletalMesh` (`self.ControlRig`) (`self.SkeletalMesh`)))