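; BP_EventManager fires scheduled random game events at BP_EventPoint actors, in offline or Strix-networked play.
; It caches the event points and game instance on begin play or sync begin, branching on a Local/Owner/Client network-role macro.
; On Tick, offline or as room owner, it steps through EventSchedule once game time drops below each entry's EventTime, rolling its probability.
; Successful rolls pick a random point, print an announcement, then start the event there after a delay.
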(event `self.ReceiveBeginPlay`
  (`self.Select_Macro`
    (:`Local`
      (bind _outactors (`GameplayStatics.GetAllActorsOfClass` "/Game/Event/BP_EventPoint.BP_EventPoint_C"))
      (set `self.EventPoints` _outactors)
      (bind _asgame_instance_main (cast `/Game/Scene/Game_Instance_Main` (`GameplayStatics.GetGameInstance`)))
      (set `self.Game Instance Main` _asgame_instance_main))))

(event `self.StrixReplicator.OnSyncBegin`
  (`self.Select_Macro`
    (:`Owner`
      _)
    (:`Client`
      _))
  (bind _outactors (`GameplayStatics.GetAllActorsOfClass` "/Game/Event/BP_EventPoint.BP_EventPoint_C"))
  (set `self.EventPoints` _outactors)
  (bind _asgame_instance_main (cast `/Game/Scene/Game_Instance_Main` (`GameplayStatics.GetGameInstance`)))
  (set `self.Game Instance Main` _asgame_instance_main))

(event `self.ReceiveTick`
  (params (DeltaSeconds :type "Float (single-precision)"))
  (bind _eventschedule (`self.EventSchedule`))
  (bind (_output_eventtime _output_eventtype _output_probability) (break `/Game/Event/EventSchedule` (`|GetArrayItem` _eventschedule (`self.count`))))
  (bind _roomowner (`self.Select_Macro`)
    (:`Local`
      ;[1 1 1] イベントが発生する時間か確認、確率で告知
      (if (not (> (`self.count`) (`KismetArrayLibrary.Array_LastIndex` _eventschedule))) :!label _label
        (bind _game_instance_main (`self.Game Instance Main`)
          (:`then`
            (if (> _output_eventtime (`/Game/Scene/Game_Instance_Main.Time` _game_instance_main))
              (`|ExecutionSequence`
                (:`then_0`
                  (if (> _output_probability (`KismetMathLibrary.RandomFloatInRange` 0.0 100.0))
                    (`self.EventAnnouncement` _output_eventtype)))
                (:`then_1`
                  (`/Engine/EditorBlueprintResources/StandardMacros.IncrementInt` (`self.count`))))))
          (:`else`))))
    (:`Owner`
      (if _roomowner
        (goto _label)))))

(event `EventAnnouncement`
  (params (eventType :type "/Game/Event/EventType Enum" :default "NewEnumerator0"))
  (set `self.Event Type` eventType)
  ;[1 1 1] 出現場所決定
  (bind _output_get (set `self.pointNum` (`KismetMathLibrary.RandomIntegerInRange` 0 (`KismetArrayLibrary.Array_LastIndex` (`self.EventPoints`)))))
  ;[1 1 1] ここでアナウンス
  (`KismetSystemLibrary.PrintString` (`KismetStringLibrary.Concat_StrStr` (`KismetStringLibrary.Conv_IntToString` (`self.delayTime`)) "秒後に" " \n場所：" (`/Game/Event/BP_EventPoint.print` (`|GetArrayItem` (`self.EventPoints`) _output_get)) " \nイベント内容：" (`|GetEnumeratorNameAsString` eventType)) true true (struct :`G` 0.66 :`B` 1.0 :`A` 1.0) (`KismetMathLibrary.Conv_IntToDouble` (`self.delayTime`)))
  (`KismetSystemLibrary.Delay` (`KismetMathLibrary.Conv_IntToDouble` (`self.delayTime`)))
  (`self.EventStart`))

(event `EventStart`
  (`/Game/Event/BP_EventPoint.EventStart` (`|GetArrayItem` (`self.EventPoints`) (`self.pointNum`)) (`self.Event Type`)))

(fn `Select`
  (returns (NetWorkType :type "/Game/Character/NetworkType Enum") (IsRoomOwner :type Boolean))
  (`|ExecutionSequence`
    (:`then_0`
      (bind _returnvalue (`StrixBlueprintFunctionLibrary.IsRoomServerConnected` 0))
      (if (not _returnvalue)
        (return "NewEnumerator0" false)))
    (:`then_1`
      (bind _strixreplicator (`self.StrixReplicator`)
        (:`then`
          (if (`StrixReplicatorComponent.GetIsOwner` _strixreplicator)
            (bind _returnvalue_2 (`StrixBlueprintFunctionLibrary.IsRoomOwner` 0))
            (return "NewEnumerator2" _returnvalue_2)
            (else
              (bind _returnvalue_3 (`StrixBlueprintFunctionLibrary.IsRoomOwner` 0))
              (return "NewEnumerator3" _returnvalue_3))))
        (:`else`)))))

(fn `UserConstructionScript`)