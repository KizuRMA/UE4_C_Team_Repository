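; BP_EventPoint is an event marker actor that spawns slimes around its location when an event starts.
; EventStart maps the event type to a fire, water, wind or metal slime class.
; Elemental mass-generation events share one loop that spawns a large batch, while the rare event spawns a single metal slime.
; Each spawn lands on a random navmesh-reachable point within a fixed radius of the actor.
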(event `EventStart`
  (params (EventType :type Byte))
  (`|ExecutionSequence`
    (:`then_0`
      (switch `/Game/Event/EventType` (cast `/Game/Event/EventType` EventType)
        (:`NewEnumerator0`
          (set `self.class` "/Game/Character/Enemy/Slime/Slime/BP_FireSlime.BP_FireSlime_C"))
        (:`NewEnumerator1`
          (set `self.class` "/Game/Character/Enemy/Slime/Slime/BP_WaterSlime.BP_WaterSlime_C"))
        (:`NewEnumerator2`
          (set `self.class` "/Game/Character/Enemy/Slime/Slime/BP_WindSlime.BP_WindSlime_C"))
        (:`NewEnumerator3`
          (set `self.class` "/Game/Character/Enemy/Slime/MetalSlime/BP_MetalSlime.BP_MetalSlime_C"))))
    (:`then_1`
      (switch `/Game/Event/EventType` (cast `/Game/Event/EventType` EventType)
        (:`NewEnumerator0`
          (for _ (range 31) :!label _label
            (`|SpawnActorFromClass` (`self.class`) (`KismetMathLibrary.MakeTransform` (`NavigationSystemV1.K2_GetRandomReachablePointInRadius` (`self.K2_GetActorLocation`) 3000.0 null null)) "Undefined" "OverrideRootScale" null null)))
        (:`NewEnumerator1`
          (goto _label))
        (:`NewEnumerator2`
          (goto _label))
        (:`NewEnumerator3`
          (`|SpawnActorFromClass` (`self.class`) (`KismetMathLibrary.MakeTransform` (`NavigationSystemV1.K2_GetRandomReachablePointInRadius` (`self.K2_GetActorLocation`) 3000.0 null null)) "Undefined" "OverrideRootScale" null null))))))

(fn `UserConstructionScript`)